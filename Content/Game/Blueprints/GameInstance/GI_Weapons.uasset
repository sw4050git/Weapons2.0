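; Game instance that manages save data, level transitions, screen fades and level BGM across the game.
; A save-data manager tracks each player's last play time and level, while per-level saves use slots keyed by player GUID and level name.
; Loaded saves bind to a save dispatcher fired by SaveGame.
; Level opens fade out first, passing the saved start tag; starting outside Title generates a debug player ID.
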(event Custom|SaveGame
  ;[1 1 1] Save
  (Default|CallEDSave)
  (bind _savedatainfo (Class|CPPSaveDataManager|GetSaveDataInfo (Variables|Default|GetSaveDataManager) (Variables|Default|GetCurrentPlayerID)))
  (bind _structout (Utilities|Struct|SetmembersinST_SaveDataInfo _savedatainfo (Math|DateTime|Now) (Variables|Default|GetCurrentLevelName) (Variables|Default|GetCurrentLevelSaveDataClass)))
  (Class|CPPSaveDataManager|UpdateSaveDataInfo (Variables|Default|GetSaveDataManager) _structout))

(event Custom|LoadLevelData
  ;[1 1 1] Load
  (bind _savegame (CallFunction|LoadWeaponsSaveGame (Utilities|String|ToString(Name) (Variables|Default|GetCurrentLevelName)) (Variables|Default|GetCurrentLevelSaveDataClass)))
  (bind _ascpp_level_save_data (Utilities|Casting|CastToCPP_LevelSaveData _savegame))
  (Variables|Default|SetCurrentLevelSaveData _ascpp_level_save_data))

(event Custom|PlayBGM
  ;[1 1 1] BGM
  (Utilities|IsValid (Variables|Default|GetCurrentLevelSaveData)
    (:Is%20Valid
      (bind _returnvalue (Audio|SpawnSound2D (Variables|/Script/Weapons.CPP_LevelSaveData|GetLevelBGM (Variables|Default|GetCurrentLevelSaveData)) 1.0 1.0 0.0 0))
      (bind _output_get (Variables|Default|SetBGM _returnvalue))
      (Utilities|IsValid _output_get
        (:Is%20Valid
          (Audio|Components|Audio|FadeIn (Variables|Default|GetBGM) 1.0 1.0 0.0 "Linear" :!class /Script/Engine.AudioComponent))))))

(event Custom|StopBGM
  ;[1 1 1] BGM
  (Utilities|IsValid (Variables|Default|GetBGM)
    (:Is%20Valid
      (Audio|Components|Audio|FadeOut (Variables|Default|GetBGM) 1.0 0.0 "Linear" :!class /Script/Engine.AudioComponent))))

(event Custom|LoadSaveDataManager
  ;[1 1 1] Load
  (bind _savegame (CallFunction|LoadSaveGame "SaveDataManeger" "/Script/Weapons.CPP_SaveDataManager"))
  (bind _ascpp_save_data_manager (Utilities|Casting|CastToCPP_SaveDataManager _savegame))
  (Variables|Default|SetSaveDataManager _ascpp_save_data_manager))

(event Custom|OpenLevelWithSaveDataLoad
  (params (LevelName :type Name) (SGLevelClass :type CPP%20Level%20Save%20Data%20Class%20Reference))
  ;[1 1 1] OpenLevel
  (Variables|Default|SetCurrentLevelName LevelName)
  (Variables|Default|SetCurrentLevelSaveDataClass SGLevelClass)
  (bind _savedatainfo (Class|CPPSaveDataManager|GetSaveDataInfo (Variables|Default|GetSaveDataManager) (Variables|Default|GetCurrentPlayerID)))
  (bind _structout (Utilities|Struct|SetmembersinST_SaveDataInfo _savedatainfo (Math|DateTime|Now) (Variables|Default|GetCurrentLevelName)))
  (Class|CPPSaveDataManager|UpdateSaveDataInfo (Variables|Default|GetSaveDataManager) _structout)
  (CallFunction|LoadLevelData)
  (CallFunction|OpenLevelwithFadeOut (Variables|Default|GetCurrentLevelName) (Utilities|String|Append "#" (Utilities|String|ToString(Name) (Variables|/Script/Weapons.CPP_LevelSaveData|GetCurrentStartTag (Variables|Default|GetCurrentLevelSaveData))))))

(event Custom|FadeInScreen
  ;[1 1 1] OpenLevel
  (CallFunction|PlayBGM)
  (Input|DisableInput (Game|GetPlayerController 0) 0)
  (bind _returnvalue (UserInterface|CreateWidget "/Game/Game/Blueprints/Widgets/Utility/WB_Fade.WB_Fade_C"))
  (bind _output_get (Variables|Default|SetFadeCover _returnvalue))
  (UserInterface|Viewport|AddtoViewport _output_get 2)
  (|PlayAnimationTimeRange (Variables|Default|GetFadeCover) (Variables|/Game/Game/Blueprints/Widgets/Utility/WB_Fade.WB_Fade_C|GetFade (Variables|Default|GetFadeCover)) 0.0 0.0 1 "Forward" 1.0
    (:Finished
      (Input|EnableInput (Game|GetPlayerController 0) 0))))

(event Custom|OpenLevelWithFadeOut
  (params (LevelName :type Name) (Option :type String))
  (bind _fadecover (Variables|Default|GetFadeCover))
  ;[1 1 1] OpenLevel
  (CallFunction|StopBGM)
  (Input|DisableInput (Game|GetPlayerController 0) 0)
  (|PlayAnimationTimeRange _fadecover (Variables|/Game/Game/Blueprints/Widgets/Utility/WB_Fade.WB_Fade_C|GetFade _fadecover) 0.0 0.0 1 "Reverse" 1.0
    (:Finished
      (Game|OpenLevel(byName) LevelName true Option))))

(event Custom|OpenTitle
  ;[1 1 1] OpenLevel
  (CallFunction|ResetCurrentData)
  (CallFunction|OpenLevelwithFadeOut "Title"))

(event EventInit
  (CallFunction|LoadSaveDataManager)
  (bind _returnvalue (Game|GetCurrentLevelName true))
  ;[1 1 1] デバッグ用
  (if (Utilities|Enum|NotEqual(Enum) _returnvalue "Title")
    (Variables|Default|SetCurrentPlayerID (Utilities|Struct|MakeGuid))
    (bind _output_get (Variables|Default|SetCurrentLevelName (Utilities|String|StringToName _returnvalue)))
    (Variables|Default|SetCurrentLevelSaveDataClass (.Value (Utilities|Map|Find (Variables|Debug|GetLevelSaveDataClasses) _output_get)))
    (CallFunction|LoadLevelData)))

(fn LoadSaveGame
  (params (SlotName :type String) (SaveGameClass :type Save%20Game%20Class%20Reference))
  (bind _returnvalue (SaveGame|DoesSaveGameExist SlotName))
  (if _returnvalue
    (bind _returnvalue_2 (SaveGame|LoadGamefromSlot SlotName))
    (return _returnvalue_2)
    (else
      (bind _returnvalue_3 (SaveGame|CreateSaveGameObject SaveGameClass))
      (SaveGame|SaveGametoSlot _returnvalue_3 SlotName)
      (return _returnvalue_3))))

(fn ResetCurrentData
  (Variables|Default|SetCurrentPlayerID (Utilities|Struct|MakeGuid))
  (Variables|Default|SetCurrentLevelSaveData 0)
  (Variables|Default|SetCurrentLevelName "None")
  (Variables|Default|SetCurrentLevelSaveDataClass 0))

(fn LoadWeaponsSaveGame
  (params (SlotType :type String) (SaveGameClass :type CPP%20Weapons%20Save%20Game%20Class%20Reference))
  (bind _currentplayerid (Variables|Default|GetCurrentPlayerID))
  (bind _returnvalue (Guid|ToString(Guid) _currentplayerid))
  (bind _returnvalue_2 (Utilities|String|Append _returnvalue "." SlotType))
  (bind _returnvalue_3 (SaveGame|DoesSaveGameExist _returnvalue_2))
  (if _returnvalue_3
    (bind _returnvalue_4 (SaveGame|LoadGamefromSlot _returnvalue_2))
    (bind _ascpp_weapons_save_game (Utilities|Casting|CastToCPP_WeaponsSaveGame _returnvalue_4))
    (LocalVariables|SetWeaponsSaveGame _ascpp_weapons_save_game)
    (else
      (bind _returnvalue_5 (SaveGame|CreateSaveGameObject SaveGameClass))
      (SaveGame|SaveGametoSlot _returnvalue_5 _returnvalue_2)
      (LocalVariables|SetWeaponsSaveGame _returnvalue_5)))
  (Variables|/Script/Weapons.CPP_WeaponsSaveGame|SetSlotName (LocalVariables|GetWeaponsSaveGame) _returnvalue_2)
  (EventDispatchers|BindEventtoEDSave (EventDispatchers|CreateEvent (LocalVariables|GetWeaponsSaveGame) :!event Save))
  (return (LocalVariables|GetWeaponsSaveGame)))