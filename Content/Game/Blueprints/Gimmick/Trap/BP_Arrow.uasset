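; Arrow trap that repeatedly fires its Box toward a target and damages Attackable actors it overlaps.
; BeginPlay loops a timed MoveComponentTo with launch and impact sounds, then teleports the Box back after a pause.
; Overlap applies GPE_Health_Recover with a negative SetByCaller magnitude through GAS, gated by a DoOnce that resets after a short cooldown.
; GetTargetLocation supplies the destination, but its TargetPoint X-offset vector is left unconnected.
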(event OnComponentBeginOverlap(Box)
  (params (OverlappedComponent :type Primitive%20Component%20Object%20Reference) (OtherActor :type Actor%20Object%20Reference) (OtherComp :type Primitive%20Component%20Object%20Reference) (OtherBodyIndex :type Integer) (bFromSweep :type Boolean) (SweepResult :type Hit%20Result%20Structure%20%28by%20ref%29))
  (bind _returnvalue (Ability|GetAbilitySystemComponent OtherActor))
  (if (Actor|ActorHasTag OtherActor "Attackable")
    (Utilities|FlowControl|DoOnce false :!label _label
      (:Completed
        (bind _returnvalue_2 (Ability|GameplayEffect|AssignTagSetbyCallerMagnitude (GameplayEffects|MakeOutgoingSpec :self _returnvalue :GameplayEffectClass "/Game/Game/Blueprints/GameplayEffect/Health/GPE_Health_Recover.GPE_Health_Recover_C") "(TagName=\"Effect.Recover.Health\")" -2e+01))
        (GameplayEffects|ApplyGameplayEffectSpecToTarget _returnvalue _returnvalue_2 _returnvalue)
        (Utilities|FlowControl|Delay 0.75)
        (goto _label Reset)))))

(event EventBeginPlay
  (Audio|PlaySoundatLocation "/Game/Game/Sounds/SwordPackUE/Stabbing/Sword_Stab_Plate__1_.Sword_Stab_Plate__1_" (Transformation|GetActorLocation) "0, 0, 0" 1.0 1.0 0.0 "/Game/Game/Sounds/SA_SE.SA_SE" 0 0 0 :!label _label)
  (Components|MoveComponentTo (Variables|Default|GetBox) (|GetTargetLocation) "0, 0, 0" false false 2.0 false)
  (Audio|PlaySoundatLocation "/Game/Game/Sounds/SwordPackUE/Slashing/Heavy_Sword_Slash_Wood__2_.Heavy_Sword_Slash_Wood__2_" (Transformation|GetActorLocation (Variables|Default|GetTargetPoint)) "0, 0, 0" 1.0 1.0 0.0 "/Game/Game/Sounds/SA_SE.SA_SE" 0 0 0)
  (Utilities|FlowControl|Delay 0.5)
  (Transformation|SetRelativeLocation (Variables|Default|GetBox) "0, 0, 0" false true)
  (goto _label))

(event Collision|EventActorBeginOverlap
  (params (OtherActor :type Actor%20Object%20Reference)))

(event EventTick
  (params (DeltaSeconds :type Float%20%28single-precision%29)))

(fn ConstructionScript)