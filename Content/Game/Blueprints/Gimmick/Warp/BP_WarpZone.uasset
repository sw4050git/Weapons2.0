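; BP_WarpZone is an interactable warp gimmick that sends the game to another level.
; On Interact it writes its PlayerStart's tag into GI_Weapons' current level save data, saves, then opens NextLevelName through a save-data load using NextSGLevelClass.
; The construction script assigns a new GUID when ID is invalid, and GetMessageText supplies the "触れる" (touch) prompt.
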(event EventInteract
  (params (CallActor :type Actor%20Object%20Reference))
  (bind _asgi_weapons (Utilities|Casting|CastToGI_Weapons (Game|GetGameInstance)))
  (Variables|/Script/Weapons.CPP_LevelSaveData|SetCurrentStartTag (Variables|/Game/Game/Blueprints/GameInstance/GI_Weapons.GI_Weapons_C|GetCurrentLevelSaveData _asgi_weapons) (Variables|/Script/Engine.PlayerStart|GetPlayerStartTag (Variables|Default|GetPlayerStart)))
  (Default|SaveGame _asgi_weapons)
  (Default|OpenLevelwithSaveDataLoad _asgi_weapons (Variables|Default|GetNextLevelName) (Variables|Default|GetNextSGLevelClass)))

(fn ConstructionScript
  (if (not (Guid|IsValidGuid (Variables|Default|GetID)))
    (Variables|Default|SetID (Guid|NewGuid))))

(fn GetMessageText
  (return "触れる"))