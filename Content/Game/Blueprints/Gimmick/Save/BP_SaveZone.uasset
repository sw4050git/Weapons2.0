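; BP_SaveZone is a rest-point gimmick that saves progress and reloads the current level when interacted with.
; Its light stays hidden until SetAvailable activates it and records its construction-generated GUID in the GI_Weapons level save data.
; BeginPlay restores that activated state from the saved IDs.
; Interact stores the linked PlayerStart's tag as the start point, saves, then reopens the level with save-data loading.
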(event Custom|SetAvailable
  (if (not (Variables|Default|GetIsAvailable))
    (Variables|Default|SetIsAvailable true)
    (Rendering|SetVisibility (Variables|Default|GetPointLight) true false)
    (bind _asgi_weapons (Utilities|Casting|CastToGI_Weapons (Game|GetGameInstance)))
    (Class|CPPLevelSaveData|AddActionedActorID (Variables|/Game/Game/Blueprints/GameInstance/GI_Weapons.GI_Weapons_C|GetCurrentLevelSaveData _asgi_weapons) (Variables|Default|GetID))))

(event EventBeginPlay
  (if (not (Variables|Default|GetIsAvailable))
    (Rendering|SetVisibility (Variables|Default|GetPointLight) false false)
    (bind _asgi_weapons (Utilities|Casting|CastToGI_Weapons (Game|GetGameInstance)))
    (Utilities|IsValid (Variables|/Game/Game/Blueprints/GameInstance/GI_Weapons.GI_Weapons_C|GetCurrentLevelSaveData _asgi_weapons)
      (:Is%20Valid
        (if (Utilities|Set|Contains (Variables|/Script/Weapons.CPP_LevelSaveData|GetActionedActorIDs (Variables|/Game/Game/Blueprints/GameInstance/GI_Weapons.GI_Weapons_C|GetCurrentLevelSaveData _asgi_weapons)) (Variables|Default|GetID))
          (Variables|Default|SetIsAvailable true)
          (Rendering|SetVisibility (Variables|Default|GetPointLight) true false))))))

(event EventInteract
  (params (CallActor :type Actor%20Object%20Reference))
  (bind _asgi_weapons (Utilities|Casting|CastToGI_Weapons (Game|GetGameInstance)))
  (Variables|/Script/Weapons.CPP_LevelSaveData|SetCurrentStartTag (Variables|/Game/Game/Blueprints/GameInstance/GI_Weapons.GI_Weapons_C|GetCurrentLevelSaveData _asgi_weapons) (Variables|/Script/Engine.PlayerStart|GetPlayerStartTag (Variables|Default|GetPlayerStart)))
  (Default|SaveGame _asgi_weapons)
  (Default|OpenLevelwithSaveDataLoad _asgi_weapons (Variables|/Game/Game/Blueprints/GameInstance/GI_Weapons.GI_Weapons_C|GetCurrentLevelName _asgi_weapons) (Variables|/Game/Game/Blueprints/GameInstance/GI_Weapons.GI_Weapons_C|GetCurrentLevelSaveDataClass _asgi_weapons)))

(fn ConstructionScript
  (if (not (Guid|IsValidGuid (Variables|Default|GetID)))
    (Variables|Default|SetID (Guid|NewGuid))))

(fn GetMessageText
  (return "休む"))