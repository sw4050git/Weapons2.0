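; BP_Gate is a gate gimmick actor that is removed when opened and stays gone through level save data.
; The construction script assigns a persistent GUID when none is valid.
; Open records that ID in the GI_Weapons game instance's current level save data and destroys the gate.
; On BeginPlay, the gate destroys itself if its ID is already recorded as actioned.
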(event Custom|Open
  (Development|PrintString "Hello")
  (bind _asgi_weapons (Utilities|Casting|CastToGI_Weapons (Game|GetGameInstance)))
  (Class|CPPLevelSaveData|AddActionedActorID (Variables|/Game/Game/Blueprints/GameInstance/GI_Weapons.GI_Weapons_C|GetCurrentLevelSaveData _asgi_weapons) (Variables|Default|GetID))
  (Actor|DestroyActor))

(event EventBeginPlay
  (bind _asgi_weapons (Utilities|Casting|CastToGI_Weapons (Game|GetGameInstance)))
  (Utilities|IsValid (Variables|/Game/Game/Blueprints/GameInstance/GI_Weapons.GI_Weapons_C|GetCurrentLevelSaveData _asgi_weapons)
    (:Is%20Valid
      (if (Utilities|Set|Contains (Variables|/Script/Weapons.CPP_LevelSaveData|GetActionedActorIDs (Variables|/Game/Game/Blueprints/GameInstance/GI_Weapons.GI_Weapons_C|GetCurrentLevelSaveData _asgi_weapons)) (Variables|Default|GetID))
        (Actor|DestroyActor)))))

(fn ConstructionScript
  (if (not (Guid|IsValidGuid (Variables|Default|GetID)))
    (Variables|Default|SetID (Guid|NewGuid))))