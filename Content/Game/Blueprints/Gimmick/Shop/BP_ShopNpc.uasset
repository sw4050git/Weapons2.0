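; Shop NPC that the player interacts with through a "話す" (Talk) prompt to talk and open a shop.
; On BeginPlay it loads a save game keyed by ShopName and initializes its lineup from a default.
; A DoOnce-guarded Interact starts the opening talk, with widget-finished delegates for sequencing the shop and closing talk.
; The lineup passes through ShopManagerSubsystem and is copied back into the save object before the closing talk.
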(event Custom|StartShop
  (Class|ShopManagerSubsystem|InitShop (Subsystems|GetShopManagerSubsystem) (Variables|/Script/Weapons.CPP_ShopSaveGame|GetShopLineup (Variables|Default|GetShopSaveGame)))
  (bind _returnvalue (UserInterface|CreateWidget "/Game/Game/Blueprints/UI/Shop/WB_Shop.WB_Shop_C"))
  (Class|BPIFPlayerController|OpenShop(Message) (Game|GetPlayerController 0) self _returnvalue)
  (EventDispatchers|BindEventtoEDFinish _returnvalue (EventDispatchers|CreateEvent :!event Custom|StartSecondTalk)))

(event Custom|StartSecondTalk
  (Default|CallEDShopFinish)
  (Variables|/Script/Weapons.CPP_ShopSaveGame|SetShopLineup (Variables|Default|GetShopSaveGame) (Variables|/Script/Weapons.ShopManagerSubsystem|GetShopLineup (Subsystems|GetShopManagerSubsystem)))
  (bind _returnvalue (UserInterface|CreateWidget "/Game/Game/Blueprints/UI/Talk/WB_Talk.WB_Talk_C" 0 (Variables|Default|GetFinishTalkAsset)))
  (Class|BPIFPlayerController|StartTalk(Message) (Game|GetPlayerController 0) _returnvalue)
  (EventDispatchers|BindEventtoEDFinished _returnvalue (EventDispatchers|CreateEvent :!event Custom|Reset)))

(event Custom|Reset
  (Utilities|FlowControl|DoOnce false) ; enters at Reset
)

(event Custom|StartFirstTalk
  (bind _returnvalue (UserInterface|CreateWidget "/Game/Game/Blueprints/UI/Talk/WB_Talk.WB_Talk_C" 0 (Variables|Default|GetStartTalkAsset)))
  (Class|BPIFPlayerController|StartTalk(Message) (Game|GetPlayerController 0) _returnvalue)
  (EventDispatchers|BindEventtoEDFinished _returnvalue (EventDispatchers|CreateEvent :!event Custom|StartShop)))

(event EventBeginPlay
  (bind _asgi_weapons (Utilities|Casting|CastToGI_Weapons (Game|GetGameInstance)))
  (bind _savegame (Default|LoadWeaponsSaveGame _asgi_weapons (Utilities|String|ToString(Name) (Variables|Default|GetShopName)) "/Script/Weapons.CPP_ShopSaveGame"))
  (bind _ascpp_shop_save_game (Utilities|Casting|CastToCPP_ShopSaveGame _savegame))
  (bind _output_get (Variables|Default|SetShopSaveGame _ascpp_shop_save_game))
  (Class|CPPShopSaveGame|InitShopLineup _output_get (Variables|Default|GetDefaultShopLineup)))

(event EventInteract
  (params (CallActor :type Actor%20Object%20Reference))
  (Utilities|FlowControl|DoOnce false
    (:Completed
      (CallFunction|StartFirstTalk))))

(fn ConstructionScript)

(fn GetMessageText
  (return "話す"))