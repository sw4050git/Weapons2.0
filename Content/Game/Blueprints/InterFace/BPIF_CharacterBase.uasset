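; Blueprint interface for base characters, defining the shared contract for action-combat behaviour without any implementation.
; It declares action calls for running, avoiding, parrying, item use, light and heavy attacks, charging, invincibility and post-death motion.
; It also exposes queries for attack state, input direction, health, stamina, magic points, weapon actor, hand location and money, plus a call to add money.
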(fn StartRunning)

(fn FinishRunning)

(fn Avoid)

(fn Parry)

(fn UseItem)

(fn LightAttack)

(fn HeavyAttack)

(fn StartCharging)

(fn SetInvincibleState
  (params (Invincible :type Boolean)))

(fn GetAttackState
  (return false))

(fn GetInputDirection
  (return "0, 0, 0"))

(fn GetStaminaValue
  (return 0.0))

(fn GetHealthValue
  (return 0.0))

(fn GetMagicPointValue
  (return 0.0))

(fn GetWeaponActor
  (return 0))

(fn GetMoney
  (return 0))

(fn AddMoney
  (params (AddValue :type Integer)))

(fn GetHandLocation
  (return "0, 0, 0"))

(fn PostDeathMotion)