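; Base character Blueprint for weapon-wielding combatants, built on the Gameplay Ability System.
; On BeginPlay it applies attack and defence maps through SetByCaller gameplay effects plus stamina effects; weapon data sets elemental attack the same way.
; Stamina-gated events activate attack, roll and parry abilities by tag, while running toggles speed and a stamina-consume tag, with a restart delay when exhausted.
; Damage and death trigger hit abilities, and an "Attackable" actor tag controls invincibility.
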(event EventBeginPlay
  ;[1 1 1] BeginPlay
  (CallFunction|ApplyAttack)
  (CallFunction|ApplyDefence)
  (GameplayEffects|ApplyGameplayEffectSpecToSelf (Variables|Default|GetAbilitySystem) (GameplayEffects|MakeOutgoingSpec :self (Variables|Default|GetAbilitySystem) :GameplayEffectClass "/Game/Game/Blueprints/GameplayEffect/Stamina/GPE_Stamina_Regenerate.GPE_Stamina_Regenerate_C"))
  (GameplayEffects|ApplyGameplayEffectSpecToSelf (Variables|Default|GetAbilitySystem) (GameplayEffects|MakeOutgoingSpec :self (Variables|Default|GetAbilitySystem) :GameplayEffectClass "/Game/Game/Blueprints/GameplayEffect/Stamina/GPE_Stamina_Consume_Run.GPE_Stamina_Consume_Run_C")))

(event EventOnDamaged
  (params (Damage :type Float%20%28single-precision%29) (Health :type Float%20%28single-precision%29) (Attacker :type Actor%20Object%20Reference))
  ;[1 1 1] Reactions
  (Variables|/Script/Engine.MovementComponent|SetVelocity (Variables|Character|GetCharacterMovement) "0, 0, 0")
  (Abilities|TryActivateAbilitiesbyTag (Variables|Default|GetAbilitySystem) (GameplayTags|MakeLiteralGameplayTagContainer "(GameplayTags=((TagName=\"Ability.Action.Hit.Damage\")))") true))

(event EventStartRunning
  (bind _returnvalue (GameplayTags|MakeLiteralGameplayTagContainer "(GameplayTags=((TagName=\"Ability.State.ConsumeStamina\"),(TagName=\"Ability.State.Run\")))"))
  (bind _returnvalue_2 (Utilities|Stamina>0))
  (bind _self self)
  ;[1 1 1] Actions
  ;;[1 1 1] Run
  (if (Math|Boolean|ANDBoolean (|Moving) _returnvalue_2 (not (|IsChargeing)))
    (Utilities|FlowControl|DoOnce false :!label _label
      (:Completed
        (Variables|/Script/Engine.CharacterMovementComponent|SetMaxWalkSpeed (Variables|Character|GetCharacterMovement) (Variables|Status|GetRunSpeed))
        (Ability|GameplayEffect|AddLooseGameplayTags _self _returnvalue)
        (goto _label_2 Reset)))
    (else
      (Utilities|FlowControl|DoOnce false :!label _label_2
        (:Completed
          (Variables|/Script/Engine.CharacterMovementComponent|SetMaxWalkSpeed (Variables|Character|GetCharacterMovement) (Variables|Status|GetDefaultWalkSpeed))
          (Ability|GameplayEffect|RemoveLooseGameplayTags _self _returnvalue)
          (if _returnvalue_2
            (goto _label Reset)
            (else
              (Utilities|FlowControl|Delay 2.0)
              (goto _label Reset))))))))

(event EventStartCharging
  ;[1 1 1] Actions
  ;;[1 1 1] HeavyAttack
  (if (Utilities|Stamina>0)
    (Abilities|TryActivateAbilitiesbyTag (Variables|Default|GetAbilitySystem) (GameplayTags|MakeLiteralGameplayTagContainer "(GameplayTags=((TagName=\"Ability.Action.Attack.Charge\")))") true)))

(event EventHeavyAttack
  ;[1 1 1] Actions
  ;;[1 1 1] HeavyAttack
  (if (Utilities|Stamina>0)
    (Abilities|TryActivateAbilitiesbyTag (Variables|Default|GetAbilitySystem) (GameplayTags|MakeLiteralGameplayTagContainer "(GameplayTags=((TagName=\"Ability.Action.Attack.Heavy\")))") true)))

(event EventLightAttack
  ;[1 1 1] Actions
  ;;[1 1 1] LightAttack
  (if (Utilities|Stamina>0)
    (Abilities|TryActivateAbilitiesbyTag (Variables|Default|GetAbilitySystem) (GameplayTags|MakeLiteralGameplayTagContainer "(GameplayTags=((TagName=\"Ability.Action.Attack.Light\")))") true)))

(event EventParry
  ;[1 1 1] Actions
  ;;[1 1 1] Parry
  (if (Utilities|Stamina>0)
    (Abilities|TryActivateAbilitiesbyTag (Variables|Default|GetAbilitySystem) (GameplayTags|MakeLiteralGameplayTagContainer "(GameplayTags=((TagName=\"Ability.Action.Parry\")))") true)))

(event EventAvoid
  ;[1 1 1] Actions
  ;;[1 1 1] Avoid
  (if (Utilities|Stamina>0)
    (Abilities|TryActivateAbilitiesbyTag (Variables|Default|GetAbilitySystem) (GameplayTags|MakeLiteralGameplayTagContainer "(GameplayTags=((TagName=\"Ability.Action.Roll\")))") true)))

(event EventOnDied
  (params (Damage :type Float%20%28single-precision%29) (Attacker :type Actor%20Object%20Reference))
  ;[1 1 1] Reactions
  (Variables|/Script/Engine.MovementComponent|SetVelocity (Variables|Character|GetCharacterMovement) "0, 0, 0")
  (Utilities|Array|RemoveItem (Variables|Default|GetTags) "Attackable")
  (Abilities|TryActivateAbilitiesbyTag (Variables|Default|GetAbilitySystem) (GameplayTags|MakeLiteralGameplayTagContainer "(GameplayTags=((TagName=\"Ability.Action.Hit.Death\")))") true))

(event EventAddMoney
  (params (AddValue :type Integer))
  (Variables|Default|SetMoney (+ (Variables|Default|GetMoney) AddValue)))

(event EventSetInvincibleState
  (params (Invincible :type Boolean))
  (bind _tags (Variables|Default|GetTags))
  ;[1 1 1] Actions
  ;;[1 1 1] Avoid
  (if Invincible
    (Utilities|Array|RemoveItem _tags "Attackable")
    (else
      (Utilities|Array|AddUnique _tags "Attackable"))))

(event EventFinishRunning
  (bind _returnvalue (GameplayTags|MakeLiteralGameplayTagContainer "(GameplayTags=((TagName=\"Ability.State.ConsumeStamina\"),(TagName=\"Ability.State.Run\")))"))
  (bind _self self)
  ;[1 1 1] Actions
  ;;[1 1 1] Run
  (Utilities|FlowControl|DoOnce false
    (:Completed
      (Variables|/Script/Engine.CharacterMovementComponent|SetMaxWalkSpeed (Variables|Character|GetCharacterMovement) (Variables|Status|GetDefaultWalkSpeed))
      (Ability|GameplayEffect|RemoveLooseGameplayTags _self _returnvalue)
      (if (Utilities|Stamina>0)
        (Utilities|FlowControl|DoOnce false) ; enters at Reset
        (else
          (Utilities|FlowControl|Delay 2.0)
          (Utilities|FlowControl|DoOnce false) ; enters at Reset
        )))))

(fn ConstructionScript)

(fn ApplyAttack
  (LocalVariables|SetSpecHandle (GameplayEffects|MakeOutgoingSpec :self (Variables|Default|GetAbilitySystem) :GameplayEffectClass "/Game/Game/Blueprints/GameplayEffect/Attack/GPE_SetAttack.GPE_SetAttack_C"))
  (bind _keys (Utilities|Map|Keys (Variables|Status|GetAttacks)))
  (for _array_element _keys
    (bind _returnvalue (Ability|GameplayEffect|AssignTagSetbyCallerMagnitude (LocalVariables|GetSpecHandle) _array_element (.Value (Utilities|Map|Find (Variables|Status|GetAttacks) _array_element))))
    (LocalVariables|SetSpecHandle _returnvalue))
  (GameplayEffects|ApplyGameplayEffectSpecToSelf (Variables|Default|GetAbilitySystem) (LocalVariables|GetSpecHandle)))

(fn ApplyDefence
  (LocalVariables|SetSpecHandle (GameplayEffects|MakeOutgoingSpec :self (Variables|Default|GetAbilitySystem) :GameplayEffectClass "/Game/Game/Blueprints/GameplayEffect/Attack/GPE_SetDefence.GPE_SetDefence_C"))
  (bind _keys (Utilities|Map|Keys (Variables|Status|GetDefences)))
  (for _array_element _keys
    (bind _returnvalue (Ability|GameplayEffect|AssignTagSetbyCallerMagnitude (LocalVariables|GetSpecHandle) _array_element (.Value (Utilities|Map|Find (Variables|Status|GetDefences) _array_element))))
    (LocalVariables|SetSpecHandle _returnvalue))
  (GameplayEffects|ApplyGameplayEffectSpecToSelf (Variables|Default|GetAbilitySystem) (LocalVariables|GetSpecHandle)))

(fn ApplyWeaponAttack
  (params (WeaponData :type CPP%20Weapon%20Data%20Asset%20Object%20Reference))
  (LocalVariables|SetTmpWeapon WeaponData)
  (bind _returnvalue (Ability|GameplayEffect|AssignTagSetbyCallerMagnitude (GameplayEffects|MakeOutgoingSpec :self (Variables|Default|GetAbilitySystem) :GameplayEffectClass "/Game/Game/Blueprints/GameplayEffect/Attack/GPE_SetAttack_Weapon.GPE_SetAttack_Weapon_C") "(TagName=\"Effect.Set.Attack.Base\")" (Variables|/Script/Weapons.CPP_WeaponDataAsset|GetAttack (LocalVariables|GetTmpWeapon))))
  (bind _returnvalue_2 (Ability|GameplayEffect|AssignTagSetbyCallerMagnitude _returnvalue "(TagName=\"Effect.Set.Attack.Flame\")" (Variables|/Script/Weapons.CPP_WeaponDataAsset|GetAttack_Flame (LocalVariables|GetTmpWeapon))))
  (bind _returnvalue_3 (Ability|GameplayEffect|AssignTagSetbyCallerMagnitude _returnvalue_2 "(TagName=\"Effect.Set.Attack.Ice\")" (Variables|/Script/Weapons.CPP_WeaponDataAsset|GetAttack_Ice (LocalVariables|GetTmpWeapon))))
  (bind _returnvalue_4 (Ability|GameplayEffect|AssignTagSetbyCallerMagnitude _returnvalue_3 "(TagName=\"Effect.Set.Attack.Mud\")" (Variables|/Script/Weapons.CPP_WeaponDataAsset|GetAttack_Mud (LocalVariables|GetTmpWeapon))))
  (bind _returnvalue_5 (Ability|GameplayEffect|AssignTagSetbyCallerMagnitude _returnvalue_4 "(TagName=\"Effect.Set.Attack.Thunder\")" (Variables|/Script/Weapons.CPP_WeaponDataAsset|GetAttack_Thunder (LocalVariables|GetTmpWeapon))))
  (bind _returnvalue_6 (Ability|GameplayEffect|AssignTagSetbyCallerMagnitude _returnvalue_5 "(TagName=\"Effect.Set.Attack.Water\")" (Variables|/Script/Weapons.CPP_WeaponDataAsset|GetAttack_Water (LocalVariables|GetTmpWeapon))))
  (bind _returnvalue_7 (Ability|GameplayEffect|AssignTagSetbyCallerMagnitude _returnvalue_6 "(TagName=\"Effect.Set.Attack.Wind\")" (Variables|/Script/Weapons.CPP_WeaponDataAsset|GetAttack_Wind (LocalVariables|GetTmpWeapon))))
  (bind _returnvalue_8 (GameplayEffects|ApplyGameplayEffectSpecToSelf (Variables|Default|GetAbilitySystem) _returnvalue_7))
  (return _returnvalue_8))

(fn GetAttackState
  (return false))

(fn GetHandLocation
  (return (Transformation|GetSocketLocation (Variables|Character|GetMesh) "HandSocket")))

(fn GetHealthValue
  (return (.ReturnValue (Ability|Attribute|GetFloatAttributefromAbilitySystemComponent (Variables|Default|GetAbilitySystem) "(AttributeName=\"Health\",Attribute=/Script/Weapons.CPP_WeaponsCharacterAttributeSet:Health,AttributeOwner=\"/Script/CoreUObject.Class'/Script/Weapons.CPP_WeaponsCharacterAttributeSet'\")"))))

(fn GetInputDirection
  (return "0, 0, 0"))

(fn GetMagicPointValue
  (return (.ReturnValue (Ability|Attribute|GetFloatAttributefromAbilitySystemComponent (Variables|Default|GetAbilitySystem) "(AttributeName=\"MagicPoint\",Attribute=/Script/Weapons.CPP_WeaponsCharacterAttributeSet:MagicPoint,AttributeOwner=\"/Script/CoreUObject.Class'/Script/Weapons.CPP_WeaponsCharacterAttributeSet'\")"))))

(fn GetMoney
  (return (Variables|Default|GetMoney)))

(fn GetStaminaValue
  (return (.ReturnValue (Ability|Attribute|GetFloatAttributefromAbilitySystemComponent (Variables|Default|GetAbilitySystem) "(AttributeName=\"Stamina\",Attribute=/Script/Weapons.CPP_WeaponsCharacterAttributeSet:Stamina,AttributeOwner=\"/Script/CoreUObject.Class'/Script/Weapons.CPP_WeaponsCharacterAttributeSet'\")"))))

(fn GetWeaponActor
  (return 0))