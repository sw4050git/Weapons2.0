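; Player controller that turns Enhanced Input into pawn movement, action messages and UI control.
; Movement is blocked by the Immovable ability tag, while other actions reach the pawn as messages.
; A slot toggle directs selection to items or weapons through the item database subsystem.
; It creates play and menu widgets, receives talk, shop and buy-menu widgets, and swaps input mapping contexts as those screens open and close.
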(event Custom|AddInputMapping
  (bind _self self)
  (bind _returnvalue (PlayerController|LocalPlayerSubsystems|GetEnhancedInputLocalPlayerSubsystem _self))
  ;[1 1 1] BeginPlay
  (Utilities|IsValid _returnvalue
    (:Is%20Valid
      (Input|AddMappingContext _returnvalue "/Game/Game/Inputs/Action/IMC_Action.IMC_Action" 0 "(bIgnoreAllPressedKeysUntilRelease=True,bForceImmediately=False,bNotifyUserSettings=False)"))))

(event Custom|SetPlayUI
  ;[1 1 1] BeginPlay
  (bind _returnvalue (UserInterface|CreateWidget "/Game/Game/Blueprints/Widgets/Play/WB_Play.WB_Play_C"))
  (bind _output_get (Variables|Default|SetPlayUI _returnvalue))
  (UserInterface|Viewport|AddtoViewport _output_get 0))

(event Custom|SetMenuUI
  ;[1 1 1] BeginPlay
  (bind _returnvalue (UserInterface|CreateWidget "/Game/Game/Blueprints/Widgets/Menu/WB_Menu.WB_Menu_C"))
  (bind _output_get (Variables|Default|SetMenuUI _returnvalue))
  (UserInterface|Viewport|AddtoViewport _output_get 1)
  (CallFunction|CloseMenu))

(event Input|EnhancedActionEvents|EnhancedInputActionIA_Action_SelectElement
  (params (ActionValue :type Float%20%28double-precision%29) (ElapsedSeconds :type Float%20%28double-precision%29) (TriggeredSeconds :type Float%20%28double-precision%29) (InputAction :type Input%20Action%20Object%20Reference :default "/Game/Game/Inputs/Action/Actions/IA_Action_SelectElement.IA_Action_SelectElement"))
  (bind _returnvalue (Subsystems|GetItemDataBaseSubsystem))
  (bind _returnvalue_2 (> ActionValue 0.0))
  ;[1 1 1] SelectItems/Weapons
  (if (Variables|Default|GetIsItemSlot)
    (Class|ItemDataBaseSubsystem|ItemSelect _returnvalue _returnvalue_2)
    (elif (|IsNotAttacking)
      (Class|ItemDataBaseSubsystem|WeaponSelect _returnvalue _returnvalue_2))))

(event Input|EnhancedActionEvents|EnhancedInputActionIA_Action_SelectSlot
  (params (ActionValue :type Float%20%28double-precision%29) (ElapsedSeconds :type Float%20%28double-precision%29) (TriggeredSeconds :type Float%20%28double-precision%29) (InputAction :type Input%20Action%20Object%20Reference :default "/Game/Game/Inputs/Action/Actions/IA_Action_SelectSlot.IA_Action_SelectSlot"))
  ;[1 1 1] SelectItems/Weapons
  (bind _isa (Utilities|FlowControl|FlipFlop)
    (:A
      _)
    (:B
      _))
  (bind _output_get (Variables|Default|SetIsItemSlot _isa))
  (Class|BPIFPlayUI|UpdateSelectSlotUI(Message) (Variables|Default|GetPlayUI) _output_get))

(event Input|EnhancedActionEvents|EnhancedInputActionIA_Menu_SelectTab
  (params (ActionValue :type Float%20%28double-precision%29) (ElapsedSeconds :type Float%20%28double-precision%29) (TriggeredSeconds :type Float%20%28double-precision%29) (InputAction :type Input%20Action%20Object%20Reference :default "/Game/Game/Inputs/Menu/Actions/IA_Menu_SelectTab.IA_Menu_SelectTab"))
  ;[1 1 1] Menu
  (Default|SwitchTab (Variables|Default|GetMenuUI) (> ActionValue 0.0)))

(event Input|EnhancedActionEvents|EnhancedInputActionIA_Shop_Close
  (params (ActionValue :type Boolean) (ElapsedSeconds :type Float%20%28double-precision%29) (TriggeredSeconds :type Float%20%28double-precision%29) (InputAction :type Input%20Action%20Object%20Reference :default "/Game/Game/Inputs/Shop/Actions/IA_Shop_Close.IA_Shop_Close"))
  ;[1 1 1] Shop
  (CallFunction|CloseShop))

(event Input|EnhancedActionEvents|EnhancedInputActionIA_Shop_SelectTab
  (params (ActionValue :type Float%20%28double-precision%29) (ElapsedSeconds :type Float%20%28double-precision%29) (TriggeredSeconds :type Float%20%28double-precision%29) (InputAction :type Input%20Action%20Object%20Reference :default "/Game/Game/Inputs/Shop/Actions/IA_Shop_SelectTab.IA_Shop_SelectTab"))
  ;[1 1 1] Shop
  (Default|SwitchTab (Variables|Default|GetShopUI) (> ActionValue 0.0)))

(event Input|EnhancedActionEvents|EnhancedInputActionIA_Action_Interact
  (params (ActionValue :type Boolean) (ElapsedSeconds :type Float%20%28double-precision%29) (TriggeredSeconds :type Float%20%28double-precision%29) (InputAction :type Input%20Action%20Object%20Reference :default "/Game/Game/Inputs/Action/Actions/IA_Action_Interact.IA_Action_Interact"))
  ;[1 1 1] Actions
  (Class|BPIFPlayer|Interact(Message) (Pawn|GetControlledPawn)))

(event Input|EnhancedActionEvents|EnhancedInputActionIA_BuyMenu_AddCount
  (params (ActionValue :type Float%20%28double-precision%29) (ElapsedSeconds :type Float%20%28double-precision%29) (TriggeredSeconds :type Float%20%28double-precision%29) (InputAction :type Input%20Action%20Object%20Reference :default "/Game/Game/Inputs/Shop/Actions/IA_BuyMenu_AddCount.IA_BuyMenu_AddCount"))
  ;[1 1 1] Shop
  (Class|BPIFBuyMenu|AddBuyCount(Message) (Variables|Default|GetBuyMenuUI) (select (> ActionValue 0.0) 1 -1)))

(event Input|EnhancedActionEvents|EnhancedInputActionIA_Talk_Finish
  (params (ActionValue :type Boolean) (ElapsedSeconds :type Float%20%28double-precision%29) (TriggeredSeconds :type Float%20%28double-precision%29) (InputAction :type Input%20Action%20Object%20Reference :default "/Game/Game/Inputs/Talk/Actions/IA_Talk_Finish.IA_Talk_Finish"))
  ;[1 1 1] Talk
  (CallFunction|FinishTalk))

(event Input|EnhancedActionEvents|EnhancedInputActionIA_Talk_ToNext
  (params (ActionValue :type Boolean) (ElapsedSeconds :type Float%20%28double-precision%29) (TriggeredSeconds :type Float%20%28double-precision%29) (InputAction :type Input%20Action%20Object%20Reference :default "/Game/Game/Inputs/Talk/Actions/IA_Talk_ToNext.IA_Talk_ToNext"))
  ;[1 1 1] Talk
  (Default|ToNext (Variables|Default|GetTalkUI)))

(event Input|EnhancedActionEvents|EnhancedInputActionIA_Talk_SelectOption
  (params (ActionValue :type Float%20%28double-precision%29) (ElapsedSeconds :type Float%20%28double-precision%29) (TriggeredSeconds :type Float%20%28double-precision%29) (InputAction :type Input%20Action%20Object%20Reference :default "/Game/Game/Inputs/Talk/Actions/IA_Talk_SelectOption.IA_Talk_SelectOption"))
  ;[1 1 1] Talk
  (Default|SelectOption (Variables|Default|GetTalkUI) (> ActionValue 0.0)))

(event Input|EnhancedActionEvents|EnhancedInputActionIA_Action_UseItem
  (params (ActionValue :type Boolean) (ElapsedSeconds :type Float%20%28double-precision%29) (TriggeredSeconds :type Float%20%28double-precision%29) (InputAction :type Input%20Action%20Object%20Reference :default "/Game/Game/Inputs/Action/Actions/IA_Action_UseItem.IA_Action_UseItem"))
  ;[1 1 1] Actions
  (Class|BPIFCharacterBase|UseItem(Message) (Pawn|GetControlledPawn)))

(event Input|EnhancedActionEvents|EnhancedInputActionIA_Action_Look
  (params (ActionValue :type Vector%202D%20Structure) (ElapsedSeconds :type Float%20%28double-precision%29) (TriggeredSeconds :type Float%20%28double-precision%29) (InputAction :type Input%20Action%20Object%20Reference :default "/Game/Game/Inputs/Action/Actions/IA_Action_Look.IA_Action_Look"))
  ;[1 1 1] Movements
  (Pawn|Input|AddControllerYawInput (Pawn|GetControlledPawn) (.x ActionValue))
  (Pawn|Input|AddControllerPitchInput (Pawn|GetControlledPawn) (.y ActionValue))
  (Class|BPIFPlayer|TargetChangewithAxisInput(Message) (Pawn|GetControlledPawn) (.x ActionValue)))

(event Input|EnhancedActionEvents|EnhancedInputActionIA_BuyMenu_Close
  (params (ActionValue :type Boolean) (ElapsedSeconds :type Float%20%28double-precision%29) (TriggeredSeconds :type Float%20%28double-precision%29) (InputAction :type Input%20Action%20Object%20Reference :default "/Game/Game/Inputs/Shop/Actions/IA_BuyMenu_Close.IA_BuyMenu_Close"))
  ;[1 1 1] Shop
  (CallFunction|CloseBuyMenu))

(event Input|EnhancedActionEvents|EnhancedInputActionIA_Action_TargetLockOn
  (params (ActionValue :type Boolean) (ElapsedSeconds :type Float%20%28double-precision%29) (TriggeredSeconds :type Float%20%28double-precision%29) (InputAction :type Input%20Action%20Object%20Reference :default "/Game/Game/Inputs/Action/Actions/IA_Action_TargetLockOn.IA_Action_TargetLockOn"))
  ;[1 1 1] Actions
  (Class|BPIFPlayer|TargetLockon(Message) (Pawn|GetControlledPawn)))

(event Input|EnhancedActionEvents|EnhancedInputActionIA_Action_Move
  (params (ActionValue :type Vector%202D%20Structure) (ElapsedSeconds :type Float%20%28double-precision%29) (TriggeredSeconds :type Float%20%28double-precision%29) (InputAction :type Input%20Action%20Object%20Reference :default "/Game/Game/Inputs/Action/Actions/IA_Action_Move.IA_Action_Move"))
  (bind _returnvalue (Pawn|GetControlledPawn))
  (bind _returnvalue_2 (Pawn|GetControlledPawn))
  (bind _returnvalue_3 (Pawn|GetControlRotation _returnvalue :!class /Script/Engine.Pawn))
  (bind _returnvalue_4 (Ability|GetAbilitySystemComponent _returnvalue_2))
  ;[1 1 1] Movements
  (Utilities|IsValid _returnvalue_4
    (:Is%20Valid
      (if (not (GameplayTags|HasMatchingGameplayTag _returnvalue_4 "(TagName=\"Ability.State.Immovable\")"))
        (Pawn|Input|AddMovementInput (Pawn|GetControlledPawn) (Math|Vector|GetRightVector (Math|Rotator|MakeRotator (.roll _returnvalue_3) 0.0 (.yaw _returnvalue_3))) (.x ActionValue) false)
        (Pawn|Input|AddMovementInput (Pawn|GetControlledPawn) (Math|Vector|GetForwardVector (Math|Rotator|MakeRotator 0.0 0.0 (.yaw (Pawn|GetControlRotation (Pawn|GetControlledPawn) :!class /Script/Engine.Pawn)))) (.y ActionValue) false)))))

(event Input|EnhancedActionEvents|EnhancedInputActionIA_Action_LightAttack
  (params (ActionValue :type Boolean) (ElapsedSeconds :type Float%20%28double-precision%29) (TriggeredSeconds :type Float%20%28double-precision%29) (InputAction :type Input%20Action%20Object%20Reference :default "/Game/Game/Inputs/Action/Actions/IA_Action_LightAttack.IA_Action_LightAttack"))
  ;[1 1 1] Actions
  (Class|BPIFCharacterBase|LightAttack(Message) (Pawn|GetControlledPawn)))

(event Input|EnhancedActionEvents|EnhancedInputActionIA_Action_HeavyAttack
  (params (ActionValue :type Boolean) (ElapsedSeconds :type Float%20%28double-precision%29) (TriggeredSeconds :type Float%20%28double-precision%29) (InputAction :type Input%20Action%20Object%20Reference :default "/Game/Game/Inputs/Action/Actions/IA_Action_HeavyAttack.IA_Action_HeavyAttack"))
  ;[1 1 1] Actions
  (:Triggered
    (Class|BPIFCharacterBase|StartCharging(Message) (Pawn|GetControlledPawn)))
  (:Started
    (Class|BPIFCharacterBase|HeavyAttack(Message) (Pawn|GetControlledPawn))))

(event Input|EnhancedActionEvents|EnhancedInputActionIA_Action_Avoid
  (params (ActionValue :type Boolean) (ElapsedSeconds :type Float%20%28double-precision%29) (TriggeredSeconds :type Float%20%28double-precision%29) (InputAction :type Input%20Action%20Object%20Reference :default "/Game/Game/Inputs/Action/Actions/IA_Action_Avoid.IA_Action_Avoid"))
  ;[1 1 1] Actions
  (Class|BPIFCharacterBase|Avoid(Message) (Pawn|GetControlledPawn)))

(event Input|EnhancedActionEvents|EnhancedInputActionIA_Action_Run
  (params (ActionValue :type Boolean) (ElapsedSeconds :type Float%20%28double-precision%29) (TriggeredSeconds :type Float%20%28double-precision%29) (InputAction :type Input%20Action%20Object%20Reference :default "/Game/Game/Inputs/Action/Actions/IA_Action_Run.IA_Action_Run"))
  (bind _returnvalue (Pawn|GetControlledPawn))
  ;[1 1 1] Actions
  (:Triggered
    (Class|BPIFCharacterBase|StartRunning(Message) _returnvalue))
  (:Completed
    (Class|BPIFCharacterBase|FinishRunning(Message) _returnvalue)))

(event Input|EnhancedActionEvents|EnhancedInputActionIA_Menu_OpenClose
  (params (ActionValue :type Boolean) (ElapsedSeconds :type Float%20%28double-precision%29) (TriggeredSeconds :type Float%20%28double-precision%29) (InputAction :type Input%20Action%20Object%20Reference :default "/Game/Game/Inputs/Menu/Actions/IA_Menu_OpenClose.IA_Menu_OpenClose"))
  ;[1 1 1] Menu
  (Utilities|FlowControl|FlipFlop
    (:A
      (CallFunction|OpenMenu))
    (:B
      (CallFunction|CloseMenu))))

(event EventBeginPlay
  ;[1 1 1] BeginPlay
  (CallFunction|AddInputMapping)
  (CallFunction|SetPlayUI)
  (CallFunction|SetMenuUI))

(event EventCloseShop
  ;[1 1 1] Shop
  (CallFunction|ChangeMappingContext "/Game/Game/Inputs/Shop/IMC_Shop.IMC_Shop" "/Game/Game/Inputs/Action/IMC_Action.IMC_Action")
  (Widget|RemovefromParent (Variables|Default|GetShopUI))
  (Variables|Default|SetShopUI 0))

(event EventOpenBuyMenu
  (params (BuyMenu :type User%20Widget%20Object%20Reference))
  ;[1 1 1] Shop
  (bind _output_get (Variables|Default|SetBuyMenuUI BuyMenu))
  (UserInterface|Viewport|AddtoViewport _output_get 0)
  (CallFunction|ChangeMappingContext "/Game/Game/Inputs/Shop/IMC_Shop.IMC_Shop" "/Game/Game/Inputs/Shop/IMC_BuyMenu.IMC_BuyMenu"))

(event EventCloseBuyMenu
  ;[1 1 1] Shop
  (Widget|RemovefromParent (Variables|Default|GetBuyMenuUI))
  (Variables|Default|SetBuyMenuUI 0)
  (CallFunction|ChangeMappingContext "/Game/Game/Inputs/Shop/IMC_BuyMenu.IMC_BuyMenu" "/Game/Game/Inputs/Shop/IMC_Shop.IMC_Shop")
  (Default|SetTab (Variables|Default|GetShopUI)))

(event EventOpenShop
  (params (CallActor :type Actor%20Object%20Reference) (ShopUI :type WB%20Shop%20Object%20Reference))
  ;[1 1 1] Shop
  (bind _output_get (Variables|Default|SetShopUI ShopUI))
  (UserInterface|Viewport|AddtoViewport _output_get 0)
  (CallFunction|ChangeMappingContext "/Game/Game/Inputs/Action/IMC_Action.IMC_Action" "/Game/Game/Inputs/Shop/IMC_Shop.IMC_Shop"))

(event EventFinishTalk
  ;[1 1 1] Talk
  (CallFunction|ChangeMappingContext "/Game/Game/Inputs/Talk/IMC_Talk.IMC_Talk" "/Game/Game/Inputs/Action/IMC_Action.IMC_Action")
  (Widget|RemovefromParent (Variables|Default|GetTalkUI))
  (Variables|Default|SetTalkUI 0))

(event EventStartTalk
  (params (TalkUI :type WB%20Talk%20Object%20Reference))
  ;[1 1 1] Talk
  (bind _output_get (Variables|Default|SetTalkUI TalkUI))
  (UserInterface|Viewport|AddtoViewport _output_get 1)
  (CallFunction|ChangeMappingContext "/Game/Game/Inputs/Action/IMC_Action.IMC_Action" "/Game/Game/Inputs/Talk/IMC_Talk.IMC_Talk"))

(event EventSetCommandMessagetoPlayUI
  (params (TargetActor :type Actor%20Object%20Reference))
  ;[1 1 1] Actions
  (bind _text (Class|BPIFInteract|GetMessageText(Message) TargetActor))
  (Class|BPIFPlayUI|ShowActionCommand(Message) (Variables|Default|GetPlayUI) _text))

(event EventCloseMenu
  ;[1 1 1] Menu
  (Widget|SetVisibility (Variables|Default|GetMenuUI) "Hidden")
  (CallFunction|ChangeMappingContext "/Game/Game/Inputs/Menu/IMC_Menu.IMC_Menu" "/Game/Game/Inputs/Action/IMC_Action.IMC_Action"))

(event EventOpenMenu
  ;[1 1 1] Menu
  (Widget|SetVisibility (Variables|Default|GetMenuUI) "Visible")
  (Default|UpdateItemsandWeapons (Variables|Default|GetMenuUI))
  (Default|FocusMenu (Variables|Default|GetMenuUI))
  (CallFunction|ChangeMappingContext "/Game/Game/Inputs/Action/IMC_Action.IMC_Action" "/Game/Game/Inputs/Menu/IMC_Menu.IMC_Menu"))

(fn ConstructionScript)

(fn ChangeMappingContext
  (params (RemoveContext :type Input%20Mapping%20Context%20Object%20Reference) (AddContext :type Input%20Mapping%20Context%20Object%20Reference))
  (bind _self self)
  (bind _returnvalue (PlayerController|LocalPlayerSubsystems|GetEnhancedInputLocalPlayerSubsystem _self))
  (Utilities|IsValid _returnvalue
    (:Is%20Valid
      (Input|RemoveMappingContext _returnvalue RemoveContext (Utilities|Struct|MakeModifyContextOptions true false false))
      (Input|AddMappingContext _returnvalue AddContext 1 (Utilities|Struct|MakeModifyContextOptions true false false)))))