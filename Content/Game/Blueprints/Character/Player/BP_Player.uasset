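; Player character Blueprint that restores money, items and weapons from a save object and writes changes back.
; An item database subsystem drives equipment: weapon updates swap the held child actor, attack Gameplay Effect and combo abilities.
; GAS also runs item and event abilities, granting them temporarily.
; It also handles overlap-based gimmick interaction with UI prompts, target lock-on with health bar display, and death leading to a game-over screen.
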(event OnTargetLockedOff(TargetSystem)
  (params (TargetActor :type Actor%20Object%20Reference))
  ;[1 1 1] Target
  (Utilities|IsValid TargetActor
    (:Is%20Valid
      (Class|BPIFEnemy|SetHealthVarVisibility(Message) TargetActor false))))

(event OnTargetLockedon(TargetSystem)
  (params (TargetActor :type Actor%20Object%20Reference))
  ;[1 1 1] Target
  (Utilities|IsValid TargetActor
    (:Is%20Valid
      (Class|BPIFEnemy|SetHealthVarVisibility(Message) TargetActor true))))

(event OnComponentBeginOverlap(Box)
  (params (OverlappedComponent :type Primitive%20Component%20Object%20Reference) (OtherActor :type Actor%20Object%20Reference) (OtherComp :type Primitive%20Component%20Object%20Reference) (OtherBodyIndex :type Integer) (bFromSweep :type Boolean) (SweepResult :type Hit%20Result%20Structure%20%28by%20ref%29))
  ;[1 1 1] Interact
  (if (Actor|ActorHasTag OtherActor "Gimmick")
    (Utilities|Array|Add (Variables|Gimmick|GetTargetGimmicks) OtherActor)
    (Class|BPIFPlayerController|SetCommandMessagetoPlayUI(Message) (Game|GetPlayerController 0) (Utilities|Array|Get(acopy) (Variables|Gimmick|GetTargetGimmicks)))))

(event OnComponentEndOverlap(Box)
  (params (OverlappedComponent :type Primitive%20Component%20Object%20Reference) (OtherActor :type Actor%20Object%20Reference) (OtherComp :type Primitive%20Component%20Object%20Reference) (OtherBodyIndex :type Integer))
  ;[1 1 1] Interact
  (if (Utilities|Array|ContainsItem (Variables|Gimmick|GetTargetGimmicks) OtherActor)
    (Utilities|Array|RemoveItem (Variables|Gimmick|GetTargetGimmicks) OtherActor)
    (Class|BPIFPlayerController|SetCommandMessagetoPlayUI(Message) (Game|GetPlayerController 0) (Utilities|Array|Get(acopy) (Variables|Gimmick|GetTargetGimmicks)))))

(event Custom|InitStatus
  ;[1 1 1] Init
  (Variables|/Script/Engine.CharacterMovementComponent|SetMaxWalkSpeed (Variables|Character|GetCharacterMovement) (Variables|Default|GetDefaultWalkSpeed))
  (Variables|Default|SetMoney (Variables|/Game/Game/Blueprints/SaveGame/Player/SG_Player.SG_Player_C|GetMoney (Variables|SaveData|GetPlayerSaveData))))

(event Custom|SetPlayerSaveData
  ;[1 1 1] SetPlayerSaveData
  (bind _asgi_weapons (Utilities|Casting|CastToGI_Weapons (Game|GetGameInstance)))
  (bind _savegame (Default|LoadWeaponsSaveGame _asgi_weapons "Player" "/Game/Game/Blueprints/SaveGame/Player/SG_Player.SG_Player_C"))
  (bind _assg_player (Utilities|Casting|CastToSG_Player _savegame))
  (Variables|SaveData|SetPlayerSaveData _assg_player))

(event Custom|BindWeaponUpdate
  ;[1 1 1] ChangeWeapon
  ;;[1 1 1] SelectedWeapon変更の際
  ;; ChangeWeaponが呼ばれるようにする
  (EventDispatchers|BindEventtoEDUpdateWeapon (Subsystems|GetItemDataBaseSubsystem) (EventDispatchers|CreateEvent :!event Custom|ChangeWeapon)))

(event Custom|ChangeWeapon
  (bind _childactor (Variables|Default|GetChildActor))
  (bind _givedcomboabilitys (Variables|Weapon|GetGivedComboAbilitys))
  ;[1 1 1] ChangeWeapon
  ;;[1 1 1 1 14] 武器のActorを手に持たせる
  (ChildActorComponent|SetChildActorClass _childactor (Variables|/Script/Weapons.CPP_WeaponDataAsset|GetWeaponClass (Accessor|GetSelectedWeapon)))
  (Actor|SetOwner (Variables|/Script/Engine.ChildActorComponent|GetChildActor _childactor) self)
  ;;[1 1 1 1 14] 武器攻撃力をGameplay Effectで設定
  (GameplayEffects|RemoveActiveGameplayEffect (Variables|Default|GetAbilitySystem) (Variables|Weapon|GetWeaponAttackEffectHandle) -1)
  (bind _effecthandle (CallFunction|ApplyWeaponAttack (Accessor|GetSelectedWeapon)))
  (Variables|Weapon|SetWeaponAttackEffectHandle _effecthandle)
  ;;[1 1 1 1 14] 武器に設定されたAbilityを付与
  (for _array_element _givedcomboabilitys
    (GameplayAbilities|ClearAbility (Variables|Default|GetAbilitySystem) _array_element))
  (Utilities|Array|Clear _givedcomboabilitys)
  (for _array_element_2 (Variables|/Script/Weapons.CPP_WeaponDataAsset|GetComboAbilitys (Accessor|GetSelectedWeapon))
    (bind _returnvalue (GameplayAbilities|GiveAbility (Variables|Default|GetAbilitySystem) _array_element_2 0 -1))
    (Utilities|Array|Add (Variables|Weapon|GetGivedComboAbilitys) _returnvalue)))

(event Custom|InitItems
  ;[1 1 1] Init
  (Utilities|FlowControl|Sequence
    (:then_0
      (for _array_element (Variables|/Game/Game/Blueprints/SaveGame/Player/SG_Player.SG_Player_C|GetItems (Variables|SaveData|GetPlayerSaveData))
        (Class|ItemDataBaseSubsystem|AddItem (Subsystems|GetItemDataBaseSubsystem) _array_element)))
    (:then_1
      (Class|ItemDataBaseSubsystem|SetEquippedItems (Subsystems|GetItemDataBaseSubsystem) (Variables|/Game/Game/Blueprints/SaveGame/Player/SG_Player.SG_Player_C|GetEquippedItems (Variables|SaveData|GetPlayerSaveData)))
      (EventDispatchers|BindEventtoEDUpdateItem (Subsystems|GetItemDataBaseSubsystem) (EventDispatchers|CreateEvent :!event Custom|UpdateSaveItemData)))))

(event Custom|InitWeapons
  ;[1 1 1] Init
  (Utilities|FlowControl|Sequence
    (:then_0
      (for _array_element (Variables|/Game/Game/Blueprints/SaveGame/Player/SG_Player.SG_Player_C|GetWeapons (Variables|SaveData|GetPlayerSaveData))
        (Class|ItemDataBaseSubsystem|AddWeapon (Subsystems|GetItemDataBaseSubsystem) _array_element)))
    (:then_1
      (Class|ItemDataBaseSubsystem|SetEquippedWeapons (Subsystems|GetItemDataBaseSubsystem) (Variables|/Game/Game/Blueprints/SaveGame/Player/SG_Player.SG_Player_C|GetEquippedWeapons (Variables|SaveData|GetPlayerSaveData)))
      (EventDispatchers|BindEventtoEDUpdateWeapon (Subsystems|GetItemDataBaseSubsystem) (EventDispatchers|CreateEvent :!event Custom|UpdateSaveWeaponData)))))

(event Custom|UpdateSaveItemData
  ;[1 1 1] SaveDataUpdate
  (Variables|/Game/Game/Blueprints/SaveGame/Player/SG_Player.SG_Player_C|SetItems (Variables|SaveData|GetPlayerSaveData) (Class|ItemDataBaseSubsystem|GetSortedItemsbyID (Subsystems|GetItemDataBaseSubsystem)))
  (Variables|/Game/Game/Blueprints/SaveGame/Player/SG_Player.SG_Player_C|SetEquippedItems (Variables|SaveData|GetPlayerSaveData) (Variables|/Script/Weapons.ItemDataBaseSubsystem|GetEquippedItems (Subsystems|GetItemDataBaseSubsystem))))

(event Custom|UpdateSaveWeaponData
  ;[1 1 1] SaveDataUpdate
  (Variables|/Game/Game/Blueprints/SaveGame/Player/SG_Player.SG_Player_C|SetWeapons (Variables|SaveData|GetPlayerSaveData) (Class|ItemDataBaseSubsystem|GetSortedWeaponsbyID (Subsystems|GetItemDataBaseSubsystem)))
  (Variables|/Game/Game/Blueprints/SaveGame/Player/SG_Player.SG_Player_C|SetEquippedWeapons (Variables|SaveData|GetPlayerSaveData) (Variables|/Script/Weapons.ItemDataBaseSubsystem|GetEquippedWeapons (Subsystems|GetItemDataBaseSubsystem))))

(event EventTargetLockon
  ;[1 1 1] Target
  (Class|TargetSystemComponent|TargetActor (Variables|Default|GetTargetSystem)))

(event EventBeginPlay
  ;[1 1 1] BeginPlay
  (|CallParentFunction)
  (CallFunction|SetPlayerSaveData)
  (CallFunction|InitStatus)
  (CallFunction|InitItems)
  (CallFunction|InitWeapons)
  (CallFunction|ChangeWeapon)
  (CallFunction|BindWeaponUpdate))

(event EventTargetChangewithAxisInput
  (params (AxisValue :type Float%20%28double-precision%29))
  ;[1 1 1] Target
  (Class|TargetSystemComponent|TargetActorwithAxisInput (Variables|Default|GetTargetSystem) AxisValue))

(event EventInteract
  (bind _targetgimmicks (Variables|Gimmick|GetTargetGimmicks))
  (bind _output (Utilities|Array|Get(acopy) _targetgimmicks))
  ;[1 1 1] Interact
  (if (not (Utilities|Array|IsEmpty (Variables|Gimmick|GetTargetGimmicks)))
    (Class|BPIFInteract|Interact(Message) _output self)
    (Utilities|IsValid _output
      (:Is%20Valid
        (Utilities|Array|Add (Variables|Gimmick|GetTargetGimmicks) _output)
        (Utilities|Array|RemoveIndex (Variables|Gimmick|GetTargetGimmicks)))
      (:Is%20Not%20Valid
        (Utilities|Array|RemoveIndex (Variables|Gimmick|GetTargetGimmicks))))
    (Class|BPIFPlayerController|SetCommandMessagetoPlayUI(Message) (Game|GetPlayerController 0) (Utilities|Array|Get(acopy) (Variables|Gimmick|GetTargetGimmicks)))))

(event EventUseItem
  (bind _returnvalue (Subsystems|GetItemDataBaseSubsystem))
  (bind _itemdata (Class|ItemDataBaseSubsystem|GetSelectedItemData _returnvalue))
  (bind _itemdata_2 (Utilities|Struct|BreakST_ItemData _itemdata))
  (bind _itemability (Variables|/Script/Weapons.CPP_ItemDataAsset|GetItemAbility _itemdata_2))
  ;[1 1 1] UseItem
  ;;[1 1 1 1 14] 選択中アイテムのAbilityをActivate
  (Utilities|IsValid _itemdata_2
    (:Is%20Valid
      (bind _returnvalue_2 (GameplayAbilities|GiveAbility (Variables|Default|GetAbilitySystem) _itemability 0 -1))
      (Variables|Item|SetGivedItemAbility _returnvalue_2)
      (bind _returnvalue_3 (Abilities|TryActivateAbilitybyClass (Variables|Default|GetAbilitySystem) _itemability true))
      (Ability|Async|WaitGameplayEventToActor 0 "(TagName=\"Ability.Action.Item.Finish\")" true
        (:then
          ;;[1 1 1 1 14] 選択中アイテムを消費
          (if _returnvalue_3
            (Class|ItemDataBaseSubsystem|ConsumeItem (Subsystems|GetItemDataBaseSubsystem))))
        (:EventReceived
          (GameplayAbilities|ClearAbility (Variables|Default|GetAbilitySystem) (Variables|Item|GetGivedItemAbility)))))))

(event EventAddMoney
  (params (AddValue :type Integer))
  ;[1 1 1] SaveDataUpdate
  (|CallParentFunction AddValue)
  (Variables|/Game/Game/Blueprints/SaveGame/Player/SG_Player.SG_Player_C|SetMoney (Variables|SaveData|GetPlayerSaveData) (Variables|Default|GetMoney)))

(event EventActivateEventAbility
  (params (EventAbility :type Gameplay%20Ability%20Class%20Reference))
  ;[1 1 1] CallEventAbility
  (bind _returnvalue (GameplayAbilities|GiveAbility (Variables|Default|GetAbilitySystem) EventAbility 0 -1))
  (Abilities|TryActivateAbilitybyClass (Variables|Default|GetAbilitySystem) EventAbility true)
  (GameplayAbilities|ClearAbility (Variables|Default|GetAbilitySystem) _returnvalue))

(event EventSetWeaponVisibility
  (params (Visible :type Boolean))
  ;[1 1 1] ChangeWeapon
  ;;[1 1 1] 武器のVisibilityを設定
  (Rendering|SetVisibility (Variables|Default|GetChildActor) Visible false))

(event EventOnDied
  (params (Damage :type Float%20%28single-precision%29) (Attacker :type Actor%20Object%20Reference))
  ;[1 1 1] Death
  (Input|SetInputModeUIOnly (Game|GetPlayerController 0) 0 "DoNotLock" false)
  (Class|BPIFPlayerController|CloseMenu(Message) (Game|GetPlayerController 0))
  (|CallParentFunction 0.0 0))

(event EventPostDeathMotion
  ;[1 1 1] Death
  (bind _returnvalue (UserInterface|CreateWidget "/Game/Game/Blueprints/UI/GameOver/WB_GameOver.WB_GameOver_C"))
  (UserInterface|Viewport|AddtoViewport _returnvalue 0)
  (Game|SetGamePaused true)
  (Actor|DestroyActor))

(event EventClearTarget
  (params (TargetActor :type Actor%20Object%20Reference))
  ;[1 1 1] Target
  (if (== TargetActor (Class|TargetSystemComponent|GetLockedonTargetActor (Variables|Default|GetTargetSystem)))
    (Class|TargetSystemComponent|TargetLockOff (Variables|Default|GetTargetSystem))))

(fn ConstructionScript)

(fn GetSelectedWeapon
  (bind _returnvalue (Subsystems|GetItemDataBaseSubsystem))
  (bind _weapondata (Class|ItemDataBaseSubsystem|GetSelectedWeaponData _returnvalue))
  (return (select (Utilities|IsValid _weapondata) _weapondata (Variables|Weapon|GetUnarmedDataAsset))))

(fn GetAttackState
  (return (GameplayTags|HasAnyMatchingGameplayTags (Variables|Default|GetAbilitySystem) (GameplayTags|MakeLiteralGameplayTagContainer "(GameplayTags=((TagName=\"Ability.State.Attack\")))"))))

(fn GetInputDirection
  (bind _returnvalue (Pawn|GetControlRotation :!class /Script/Engine.Pawn))
  (bind _returnvalue_2 (Input|EnhancedActionValues|GetIA_Action_Move))
  (return (Math|Vector|Normalize (+ (* (Math|Vector|GetRightVector (Math|Rotator|MakeRotator (.roll _returnvalue) 0.0 (.yaw _returnvalue))) (.x _returnvalue_2)) (* (Math|Vector|GetForwardVector (Math|Rotator|MakeRotator 0.0 0.0 (.yaw _returnvalue))) (.y _returnvalue_2))))))

(fn GetWeaponActor
  (return (Variables|/Script/Engine.ChildActorComponent|GetChildActor (Variables|Default|GetChildActor))))

(fn GetTargetActor
  (return (Class|TargetSystemComponent|GetLockedonTargetActor (Variables|Default|GetTargetSystem))))