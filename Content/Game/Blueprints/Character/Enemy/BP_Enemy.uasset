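; Base enemy character that equips its weapon and combo abilities, shows a health bar briefly when hit, and alerts its controller to damage.
; Tick toggles walk speed with the Ability.State.Immovable gameplay tag.
; Death stops AI, then after the death motion awards money and drops items and weapons on traced ground.
; Non-respawnable enemies record their construction-time GUID in level save data on death and destroy themselves on later BeginPlay.
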(event Custom|SetWeapon
  (bind _childactor (Variables|Default|GetChildActor))
  ;[1 1 1] Weapon
  (ChildActorComponent|SetChildActorClass _childactor (Variables|/Script/Weapons.CPP_WeaponDataAsset|GetWeaponClass (Variables|Default|GetWeapon)))
  (Actor|SetOwner (Variables|/Script/Engine.ChildActorComponent|GetChildActor _childactor) self)
  (CallFunction|ApplyWeaponAttack (Variables|Default|GetWeapon))
  (for _array_element (Variables|/Script/Weapons.CPP_WeaponDataAsset|GetComboAbilitys (Variables|Default|GetWeapon))
    (GameplayAbilities|GiveAbility (Variables|Default|GetAbilitySystem) _array_element 0 -1)))

(event Custom|ItemDrop
  ;[1 1 1] Drop
  (Utilities|IsValid (.ItemData (Utilities|Struct|BreakST_ItemData (Variables|Drop|GetDropItem)))
    (:Is%20Valid
      (bind _location (CallFunction|GetActorUnderLocation))
      (Game|SpawnActorfromClass "/Game/Game/Blueprints/Stuff/Item/PickUps/BP_PickUpItem.BP_PickUpItem_C" (Math|Transform|MakeTransform _location (Transformation|GetActorRotation) "1.000000,1.000000,1.000000") "Undefined" "MultiplyWithRoot" 0 (Variables|Drop|GetDropItem) false 0))))

(event Custom|WeaponDrop
  ;[1 1 1] Drop
  (Utilities|IsValid (Variables|Drop|GetDropWeapon)
    (:Is%20Valid
      (bind _location (CallFunction|GetActorUnderLocation))
      (Game|SpawnActorfromClass "/Game/Game/Blueprints/Stuff/Weapon/PickUps/BP_PickUpWeapon_Box.BP_PickUpWeapon_Box_C" (Math|Transform|MakeTransform _location (Transformation|GetActorRotation) "1.000000,1.000000,1.000000") "Undefined" "MultiplyWithRoot" 0 (Variables|Drop|GetDropWeapon) false 0))))

(event Custom|InitHealthBar
  ;[1 1 1] HealthBar
  (bind _aswb_enemy_health (Utilities|Casting|CastToWB_EnemyHealth (UserInterface|GetUserWidgetObject (Variables|Default|GetWidget))))
  (Variables|HealthBar|SetEnemyHealthBar _aswb_enemy_health)
  (Variables|/Game/Game/Blueprints/UI/Enemy/WB_EnemyHealth.WB_EnemyHealth_C|SetHealth _aswb_enemy_health (.ReturnValue (Ability|Attribute|GetFloatAttributefromAbilitySystemComponent (Variables|Default|GetAbilitySystem) "(AttributeName=\"Health\",Attribute=/Script/Weapons.CPP_WeaponsCharacterAttributeSet:Health,AttributeOwner=\"/Script/CoreUObject.Class'/Script/Weapons.CPP_WeaponsCharacterAttributeSet'\")"))))

(event Custom|SetHealthVarDamageVisible
  ;[1 1 1] HealthBar
  (Widget|SetVisibility (Variables|HealthBar|GetEnemyHealthBar) "Visible")
  (Utilities|FlowControl|Delay 1e+01)
  (if (not (Variables|HealthBar|GetIsHealthBarVisible))
    (Widget|SetVisibility (Variables|HealthBar|GetEnemyHealthBar) "Hidden")))

(event Custom|CheckRespawn
  ;[1 1 1] Respawn
  (if (not (Variables|Default|GetIsRespawnable))
    (bind _asgi_weapons (Utilities|Casting|CastToGI_Weapons (Game|GetGameInstance)))
    (Utilities|IsValid (Variables|/Game/Game/Blueprints/GameInstance/GI_Weapons.GI_Weapons_C|GetCurrentLevelSaveData _asgi_weapons)
      (:Is%20Valid
        (if (Utilities|Set|Contains (Variables|/Script/Weapons.CPP_LevelSaveData|GetActionedActorIDs (Variables|/Game/Game/Blueprints/GameInstance/GI_Weapons.GI_Weapons_C|GetCurrentLevelSaveData _asgi_weapons)) (Variables|Default|GetID))
          (Actor|DestroyActor))))))

(event Custom|AddActionedActor
  ;[1 1 1] Respawn
  (if (not (Variables|Default|GetIsRespawnable))
    (bind _asgi_weapons (Utilities|Casting|CastToGI_Weapons (Game|GetGameInstance)))
    (Class|CPPLevelSaveData|AddActionedActorID (Variables|/Game/Game/Blueprints/GameInstance/GI_Weapons.GI_Weapons_C|GetCurrentLevelSaveData _asgi_weapons) (Variables|Default|GetID))))

(event EventBeginPlay
  ;[1 1 1] Default
  (CallFunction|CheckRespawn)
  (|CallParentFunction)
  (CallFunction|SetWeapon)
  (CallFunction|InitHealthBar))

(event EventPostDeathMotion
  ;[1 1 1] Death
  (Class|BPIFCharacterBase|AddMoney(Message) (Game|GetPlayerCharacter 0) (Variables|Default|GetMoney))
  (CallFunction|ItemDrop)
  (CallFunction|WeaponDrop)
  (Default|CallEDDied self)
  (Actor|DestroyActor))

(event EventSetHealthVarVisibility
  (params (Visible :type Boolean))
  ;[1 1 1] HealthBar
  (bind _output_get (Variables|HealthBar|SetIsHealthBarVisible Visible))
  (Widget|SetVisibility (Variables|HealthBar|GetEnemyHealthBar) (select _output_get "Visible" "Hidden")))

(event EventOnDamaged
  (params (Damage :type Float%20%28single-precision%29) (Health :type Float%20%28single-precision%29) (Attacker :type Actor%20Object%20Reference))
  ;[1 1 1] Damage
  (|CallParentFunction Damage Health 0)
  (Variables|/Game/Game/Blueprints/UI/Enemy/WB_EnemyHealth.WB_EnemyHealth_C|SetHealth (Variables|HealthBar|GetEnemyHealthBar) Health)
  (CallFunction|SetHealthVarDamageVisible)
  (Class|BPIFEnemyController|SetDamageFind(Message) (Pawn|GetController)))

(event EventOnDied
  (params (Damage :type Float%20%28single-precision%29) (Attacker :type Actor%20Object%20Reference))
  (bind _self self)
  (bind _returnvalue (AI|GetAIController _self))
  ;[1 1 1] Death
  (AI|Logic|StopLogic (Variables|/Script/AIModule.AIController|GetBrainComponent _returnvalue) "")
  (AI|ClearFocus _returnvalue)
  (Class|BPIFPlayer|ClearTarget(Message) self (Game|GetPlayerCharacter 0))
  (Widget|SetVisibility (Variables|HealthBar|GetEnemyHealthBar) "Collapsed")
  (CallFunction|AddActionedActor)
  (|CallParentFunction 0.0 0))

(event EventTick
  (params (DeltaSeconds :type Float%20%28single-precision%29))
  ;[1 1 1] Default
  (if (not (GameplayTags|HasMatchingGameplayTag (Variables|Default|GetAbilitySystem) "(TagName=\"Ability.State.Immovable\")"))
    (Utilities|FlowControl|DoOnce false :!label _label
      (:Completed
        (Variables|/Script/Engine.CharacterMovementComponent|SetMaxWalkSpeed (Variables|Character|GetCharacterMovement) 6e+02)
        (goto _label_2 Reset)))
    (else
      (Utilities|FlowControl|DoOnce false :!label _label_2
        (:Completed
          (Variables|/Script/Engine.CharacterMovementComponent|SetMaxWalkSpeed (Variables|Character|GetCharacterMovement) 0.0)
          (goto _label Reset))))))

(fn ConstructionScript
  (if (not (Guid|IsValidGuid (Variables|Default|GetID)))
    (Variables|Default|SetID (Guid|NewGuid))))

(fn GetInputDirection
  (bind _returnvalue (Game|GetPlayerCharacter 0))
  (bind _returnvalue_2 (Transformation|GetActorLocation))
  (bind _returnvalue_3 (Math|Float|MakeLiteralFloat 2.7e+02))
  (bind _returnvalue_4 (Transformation|GetActorLocation _returnvalue))
  (bind _returnvalue_5 (Math|Vector|GetUnitDirection(Vector) _returnvalue_4 _returnvalue_2))
  (bind (_x _y) (Math|Vector|BreakVector _returnvalue_5))
  (return (Math|Vector|RotateVectorAroundAxis (Math|Vector|MakeVector _x _y 0.0) (- (* (Math|Random|RandomFloat) _returnvalue_3) (/ _returnvalue_3 2.0)) "0.000000,0.000000,1.000000")))

(fn GetWeaponActor
  (return (Variables|/Script/Engine.ChildActorComponent|GetChildActor (Variables|Default|GetChildActor))))

(fn GetActorUnderLocation
  (bind _returnvalue (Transformation|GetActorLocation))
  (bind _outhit (Collision|LineTraceByChannel _returnvalue (- _returnvalue "0.000000,0.000000,400.000000") "TraceTypeQuery1" false (Utilities|Array|MakeArray self) "None"))
  (return (.Location (Collision|BreakHitResult _outhit))))

(fn GetAvoidProbability
  (return (Variables|AI|GetAvoidProbability)))

(fn GetCooltimeRange
  (return (Variables|AI|GetCoolTimeRange)))

(fn IsTargetable
  (return true))