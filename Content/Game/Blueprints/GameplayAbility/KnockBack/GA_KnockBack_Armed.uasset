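; GA_KnockBack_Armed is a gameplay ability that plays a hit-reaction montage (AM_Hit_F) on the owner, apparently for an armed knockback.
; Montage notify begin and end events look up a Notifys map to add and remove non-replicated loose gameplay tags on the owning actor.
; The ability ends when the montage completes, blends out or is interrupted.
; On end, it removes every mapped tag as cleanup.
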(event Ability|EventActivateAbility
  (Ability|CommitAbility)
  (bind _notifyname (Animation|Montage|PlayMontage (Class|GameplayAbility|GetOwningComponentfromActorInfo) "/Game/Game/Animations/Armed/Hit/AM_Hit_F.AM_Hit_F")
    (:OnCompleted
      (Ability|EndAbility :!label _label))
    (:OnBlendOut
      (goto _label))
    (:OnInterrupted
      (goto _label))
    (:OnNotifyBegin
      (if (.ReturnValue (Utilities|Map|Find (Variables|Default|GetNotifys) _notifyname))
        (Ability|GameplayEffect|AddLooseGameplayTags (Ability|GetOwningActorfromActorInfo) (.Value (Utilities|Map|Find (Variables|Default|GetNotifys) _notifyname)))))
    (:OnNotifyEnd
      (if (.ReturnValue (Utilities|Map|Find (Variables|Default|GetNotifys) _notifyname))
        (Ability|GameplayEffect|RemoveLooseGameplayTags (Ability|GetOwningActorfromActorInfo) (.Value (Utilities|Map|Find (Variables|Default|GetNotifys) _notifyname)))))))

(event Ability|EventOnEndAbility
  (params (bWasCancelled :type Boolean))
  (bind _values (Utilities|Map|Values (Variables|Default|GetNotifys)))
  (for _array_element _values
    (Ability|GameplayEffect|RemoveLooseGameplayTags (Ability|GetOwningActorfromActorInfo) _array_element)))