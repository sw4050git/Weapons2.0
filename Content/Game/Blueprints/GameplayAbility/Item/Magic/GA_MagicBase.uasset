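; Base Gameplay Ability for magic items that spends magic points to play a casting montage and spawn a magic actor.
; If the MP check passes, it applies Cost through a SetByCaller effect and hides the weapon.
; The SpawnMagic notify spawns MagicActor, while other notifies toggle loose tags mapped in Notifys.
; Ending the ability sends an item-finish event, restores the weapon and clears those tags.
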(event Ability|EventActivateAbility
  (bind _returnvalue (Ability|GetOwningActorfromActorInfo))
  (Ability|CommitAbility)
  (if (|MP>0)
    (bind _returnvalue_2 (Ability|GameplayEffect|AssignTagSetbyCallerMagnitude (Ability|MakeOutgoingGameplayEffectSpec "/Game/Game/Blueprints/GameplayEffect/MagicPoint/GPE_MagicPoint_Consume.GPE_MagicPoint_Consume_C") "(TagName=\"Effect.Consume.MagicPoint\")" (* (Variables|Default|GetCost) -1.0)))
    (Ability|ApplyGameplayEffectSpecToOwner _returnvalue_2)
    (Class|BPIFPlayer|SetWeaponVisibility(Message) (Ability|GetOwningActorfromActorInfo) false)
    (bind _notifyname (Animation|Montage|PlayMontage (Class|GameplayAbility|GetOwningComponentfromActorInfo) (Variables|Default|GetMontage))
      (:OnCompleted
        (Ability|EndAbility :!label _label))
      (:OnBlendOut
        (goto _label))
      (:OnInterrupted
        (goto _label))
      (:OnNotifyBegin
        (if (== _notifyname "SpawnMagic")
          (Game|SpawnActorfromClass (Variables|Default|GetMagicActor) (Transformation|GetActorTransform _returnvalue) "Undefined" "MultiplyWithRoot" 0 _returnvalue 0)
          (elif (.ReturnValue (Utilities|Map|Find (Variables|Default|GetNotifys) _notifyname))
            (Ability|GameplayEffect|AddLooseGameplayTags (Ability|GetOwningActorfromActorInfo) (.Value (Utilities|Map|Find (Variables|Default|GetNotifys) _notifyname))))))
      (:OnNotifyEnd
        (if (.ReturnValue (Utilities|Map|Find (Variables|Default|GetNotifys) _notifyname))
          (Ability|GameplayEffect|RemoveLooseGameplayTags (Ability|GetOwningActorfromActorInfo) (.Value (Utilities|Map|Find (Variables|Default|GetNotifys) _notifyname))))))
    (else
      (Ability|EndAbility))))

(event Ability|EventOnEndAbility
  (params (bWasCancelled :type Boolean))
  (Ability|SendGameplayEventtoActor (Ability|GetOwningActorfromActorInfo) "(TagName=\"Ability.Action.Item.Finish\")")
  (Class|BPIFPlayer|SetWeaponVisibility(Message) (Ability|GetOwningActorfromActorInfo) true)
  (bind _values (Utilities|Map|Values (Variables|Default|GetNotifys)))
  (for _array_element _values
    (Ability|GameplayEffect|RemoveLooseGameplayTags (Ability|GetOwningActorfromActorInfo) _array_element)))