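; Gameplay ability for a magic recovery item that plays a drink montage on its owner, hiding the weapon while active.
; The "Drink" notify applies a magic point recovery effect with a SetByCaller magnitude.
; Other notifies add and remove mapped loose gameplay tags for their duration.
; Ending the ability restores the weapon, clears those tags and sends an item-finish event to the owner.
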(event Ability|EventActivateAbility
  (Ability|CommitAbility)
  (Class|BPIFPlayer|SetWeaponVisibility(Message) (Ability|GetOwningActorfromActorInfo) false)
  (bind _notifyname (Animation|Montage|PlayMontage (Class|GameplayAbility|GetOwningComponentfromActorInfo) (Variables|Default|GetMontage))
    (:OnCompleted
      (Ability|EndAbility :!label _label))
    (:OnBlendOut
      (goto _label))
    (:OnInterrupted
      (goto _label))
    (:OnNotifyBegin
      (if (== _notifyname "Drink")
        (bind _returnvalue (Ability|GameplayEffect|AssignTagSetbyCallerMagnitude (Ability|MakeOutgoingGameplayEffectSpec "/Game/Game/Blueprints/GameplayEffect/MagicPoint/GPE_MagicPoint_Recover.GPE_MagicPoint_Recover_C") "(TagName=\"Effect.Recover.MagicPoint\")" (Variables|Default|GetRecoverValue)))
        (Ability|ApplyGameplayEffectSpecToOwner _returnvalue)
        (elif (.ReturnValue (Utilities|Map|Find (Variables|Default|GetNotifys) _notifyname))
          (Ability|GameplayEffect|AddLooseGameplayTags (Ability|GetOwningActorfromActorInfo) (.Value (Utilities|Map|Find (Variables|Default|GetNotifys) _notifyname))))))
    (:OnNotifyEnd
      (if (.ReturnValue (Utilities|Map|Find (Variables|Default|GetNotifys) _notifyname))
        (Ability|GameplayEffect|RemoveLooseGameplayTags (Ability|GetOwningActorfromActorInfo) (.Value (Utilities|Map|Find (Variables|Default|GetNotifys) _notifyname)))))))

(event Ability|EventOnEndAbility
  (params (bWasCancelled :type Boolean))
  (Ability|SendGameplayEventtoActor (Ability|GetOwningActorfromActorInfo) "(TagName=\"Ability.Action.Item.Finish\")")
  (Class|BPIFPlayer|SetWeaponVisibility(Message) (Ability|GetOwningActorfromActorInfo) true)
  (bind _values (Utilities|Map|Values (Variables|Default|GetNotifys)))
  (for _array_element _values
    (Ability|GameplayEffect|RemoveLooseGameplayTags (Ability|GetOwningActorfromActorInfo) _array_element)))