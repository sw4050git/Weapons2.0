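; Base gameplay ability for a directional roll that costs stamina and ends at once when there is no input direction.
; It converts the input's angle relative to actor forward into one of eight montages.
; Motion Warping targets a point a set distance along the input, keeping the actor's rotation.
; A SetByCaller effect deducts stamina, and ending the ability always applies a stamina regeneration cooldown effect.
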(event Ability|EventActivateAbility
  (bind _returnvalue (Ability|GetOwningActorfromActorInfo))
  (bind _returnvalue_2 (Transformation|GetActorForwardVector _returnvalue))
  (Ability|CommitAbility)
  ;[1 1 1] 入力方向を取得
  (bind _inputdirection (Class|BPIFCharacterBase|GetInputDirection(Message) (Ability|GetOwningActorfromActorInfo)))
  (bind _output_get (Variables|Default|SetInputDirection _inputdirection))
  (if (Math|Vector|VectorIsZero _output_get)
    ;[1 1 1] 入力がない場合
    (Ability|EndAbility)
    (else
      ;[1 1 1] プレイヤー前方と入力方向のなす角をSet
      (Variables|Default|SetRelativeInputAngle (Class|KismetMathLibrary|DegAcos (Math|Vector|DotProduct _returnvalue_2 (Variables|Default|GetInputDirection))))
      ;[1 1 1] なす角を時計回り正, 区間[0, 360)に変換
      (if (> (Math|Vector|DotProduct (Transformation|GetActorUpVector (Ability|GetOwningActorfromActorInfo)) (Math|Vector|CrossProduct _returnvalue_2 (Variables|Default|GetInputDirection))) 0.0)
        _
        (else
          (bind _output_get_2 (Variables|Default|SetRelativeInputAngle (+ (* (Variables|Default|GetRelativeInputAngle) -1.0) 3.6e+02)))))
      (bind _montagetoplay (|SetMontageToPlay _output_get_2))
      ;[1 1 1] 移動先のTransformを設定
      (Class|MotionWarpingComponent|AddorUpdateWarpTargetfromLocationandRotation (Actor|GetComponentbyClass (Ability|GetOwningActorfromActorInfo) "/Script/MotionWarping.MotionWarpingComponent") "Roll" (+ (* (Variables|Default|GetInputDirection) (Variables|Default|GetMovingDistance)) (Transformation|GetActorLocation (Ability|GetOwningActorfromActorInfo))) (Transformation|GetActorRotation (Ability|GetOwningActorfromActorInfo)))
      (|ConsumeStamina)
      (Animation|Montage|PlayMontage (Class|GameplayAbility|GetOwningComponentfromActorInfo) _montagetoplay
        (:OnCompleted
          _)
        (:OnBlendOut
          _)
        (:OnInterrupted
          _))
      (Ability|EndAbility))))

(event Ability|EventOnEndAbility
  (params (bWasCancelled :type Boolean))
  (Ability|ApplyGameplayEffectToOwner "/Game/Game/Blueprints/GameplayEffect/Stamina/GPE_Stamina_Regenerate_Cooldown.GPE_Stamina_Regenerate_Cooldown_C"))