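; GA_Parry is a Gameplay Ability that performs a parry by playing the AM_Parry montage on the owner's mesh.
; A "Ready" montage notify window adds and removes the loose, non-replicated Ability.Ready.Parry tag, marking when the parry is active.
; The ability ends when the montage completes, blends out or is interrupted, and clears the tag on end as a safeguard.
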(event Ability|EventActivateAbility
  (Ability|CommitAbility)
  (bind _notifyname (Animation|Montage|PlayMontage (Class|GameplayAbility|GetOwningComponentfromActorInfo) "/Game/Game/Animations/Armed/Parry/AM_Parry.AM_Parry")
    (:OnCompleted
      (Ability|EndAbility :!label _label))
    (:OnBlendOut
      (goto _label))
    (:OnInterrupted
      (goto _label))
    (:OnNotifyBegin
      (if (== _notifyname "Ready")
        (Ability|GameplayEffect|AddLooseGameplayTags (Ability|GetOwningActorfromActorInfo) (GameplayTags|MakeLiteralGameplayTagContainer "(GameplayTags=((TagName=\"Ability.Ready.Parry\")))"))))
    (:OnNotifyEnd
      (if (== _notifyname "Ready")
        (Ability|GameplayEffect|RemoveLooseGameplayTags (Ability|GetOwningActorfromActorInfo) (GameplayTags|MakeLiteralGameplayTagContainer "(GameplayTags=((TagName=\"Ability.Ready.Parry\")))"))))))

(event Ability|EventOnEndAbility
  (params (bWasCancelled :type Boolean))
  (Ability|GameplayEffect|RemoveLooseGameplayTags (Ability|GetOwningActorfromActorInfo) (GameplayTags|MakeLiteralGameplayTagContainer "(GameplayTags=((TagName=\"Ability.Ready.Parry\")))")))