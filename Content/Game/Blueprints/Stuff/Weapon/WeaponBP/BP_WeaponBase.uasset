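; Base weapon actor that deals melee hits through the Gameplay Ability System using a capsule collider that is switched on and off by attack collision events.
; On overlap, it checks for an "Attackable" tag and a different class from its owner, then whether the target has the parry-ready tag and faces the weapon.
; A parry activates the owner's hit-break ability; otherwise it applies the attack gameplay effect to the target and disables the capsule.
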(event OnComponentBeginOverlap(Capsule)
  (params (OverlappedComponent :type Primitive%20Component%20Object%20Reference) (OtherActor :type Actor%20Object%20Reference) (OtherComp :type Primitive%20Component%20Object%20Reference) (OtherBodyIndex :type Integer) (bFromSweep :type Boolean) (SweepResult :type Hit%20Result%20Structure%20%28by%20ref%29))
  (bind _returnvalue (Components|GetOwner))
  (bind _returnvalue_2 (Ability|GetAbilitySystemComponent _returnvalue))
  (if (|CheckAttackable OtherActor)
    (if (|CheckParried OtherActor)
      (Abilities|TryActivateAbilitiesbyTag (Ability|GetAbilitySystemComponent (Components|GetOwner)) (GameplayTags|MakeLiteralGameplayTagContainer "(GameplayTags=((TagName=\"Ability.Action.Hit.Break\")))") true)
      (else
        (GameplayEffects|ApplyGameplayEffectSpecToTarget _returnvalue_2 (GameplayEffects|MakeOutgoingSpec :self _returnvalue_2 :GameplayEffectClass "/Game/Game/Blueprints/GameplayEffect/Attack/GPE_Attack.GPE_Attack_C") (Ability|GetAbilitySystemComponent OtherActor))
        (Collision|SetCollisionEnabled (Variables|Default|GetCapsule) "NoCollision")))))

(event EventDeactivateAttackCollision
  (Collision|SetCollisionEnabled (Variables|Default|GetCapsule) "NoCollision"))

(event EventActivateAttackCollision
  (Collision|SetCollisionEnabled (Variables|Default|GetCapsule) "QueryAndPhysics"))

(fn ConstructionScript)