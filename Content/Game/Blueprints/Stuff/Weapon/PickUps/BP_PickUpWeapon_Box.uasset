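; Weapon pickup actor that the player can interact with to acquire a weapon.
; On Interact, it adds its Weapon to the ItemDataBaseSubsystem, calls Actioned, then destroys itself.
; GetMessageText supplies the Japanese prompt "拾う" (pick up) as hardcoded text.
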(event EventBeginPlay
  (|CallParentFunction) ; This node is disabled and will not be called.\nDrag off pins to build functionality.
)

(event Collision|EventActorBeginOverlap
  (params (OtherActor :type Actor%20Object%20Reference)))

(event EventTick
  (params (DeltaSeconds :type Float%20%28single-precision%29)))

(event EventInteract
  (params (CallActor :type Actor%20Object%20Reference))
  (Class|ItemDataBaseSubsystem|AddWeapon (Subsystems|GetItemDataBaseSubsystem) (Variables|Default|GetWeapon))
  (CallFunction|Actioned)
  (Actor|DestroyActor))

(fn ConstructionScript
  (|CallParentFunction))

(fn GetMessageText
  (return "拾う"))