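; Thunder spell actor that snaps to the ground under the caster's target, or along the caster's forward line without one, and self-destructs if no ground is found.
; Niagara exports particle data back to the Blueprint, which capsule-traces each particle for "Attackable" actors other than the caster.
; Damage reuses the health-recover GameplayEffect with negative magnitude, gated by one actor-wide cooldown shared across victims.
; The actor destroys itself when the Niagara system finishes.
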(event OnSystemFinished(Niagara)
  (params (PSystem :type Niagara%20Component%20Object%20Reference))
  (Actor|DestroyActor))

(event Custom|ApplyDamage
  (params (ACS :type Ability%20System%20Component%20Object%20Reference))
  (Utilities|FlowControl|DoOnce false :!label _label
    (:Completed
      (bind _returnvalue (Ability|GameplayEffect|AssignTagSetbyCallerMagnitude (GameplayEffects|MakeOutgoingSpec :self ACS :GameplayEffectClass "/Game/Game/Blueprints/GameplayEffect/Health/GPE_Health_Recover.GPE_Health_Recover_C") "(TagName=\"Effect.Recover.Health\")" -3e+01))
      (GameplayEffects|ApplyGameplayEffectSpecToTarget ACS _returnvalue ACS)
      (Utilities|FlowControl|Delay 0.75)
      (goto _label Reset))))

(event EventBeginPlay
  (|CallParentFunction)
  (Class|NiagaraComponent|SetVariableObject (Variables|Default|GetNiagara) "BPCallback" self)
  (Utilities|IsValid (Variables|Default|GetCaller)
    (:Is%20Valid
      (bind _targetactor (Class|BPIFPlayer|GetTargetActor(Message) (Variables|Default|GetCaller)))
      (Utilities|IsValid _targetactor
        (:Is%20Valid
          (Variables|Default|SetSpawnLocation (Transformation|GetActorLocation _targetactor)))
        (:Is%20Not%20Valid
          (bind _location (CallFunction|GetNoneTargetSpawnLocation))
          (Variables|Default|SetSpawnLocation _location)))
      (bind (_outhit _returnvalue) (Collision|LineTraceByChannel (Variables|Default|GetSpawnLocation) (- (Variables|Default|GetSpawnLocation) "0.000000,0.000000,200.000000") "TraceTypeQuery1" false (Utilities|Array|MakeArray _targetactor) "None"))
      (if _returnvalue
        (Transformation|SetActorLocation (+ (.Location (Collision|BreakHitResult _outhit)) "0.000000,0.000000,10.000000") false false)
        (else
          (Actor|DestroyActor))))))

(event EventParticleData
  (params (Data :type Array%20of%20Basic%20Particle%20Data%20Structures) (NiagaraSystem :type Niagara%20System%20Object%20Reference) (SimulationPositionOffset :type Vector%20%28by%20ref%29 :default "0, 0, 0"))
  (for _array_element Data
    (bind _outhits (Class|KismetSystemLibrary|CapsuleTraceMulti (.Position (Utilities|Struct|BreakBasicParticleData _array_element)) (+ (.Position (Utilities|Struct|BreakBasicParticleData _array_element)) (* (.Velocity (Utilities|Struct|BreakBasicParticleData _array_element)) 0.01)) 1e+02 1e+03 "TraceTypeQuery3" false 0 "ForOneFrame" true))
    (for _array_element_2 _outhits
      (if (and (Actor|ActorHasTag (.HitActor (Collision|BreakHitResult _array_element_2)) "Attackable") (!= (Variables|Default|GetCaller) (.HitActor (Collision|BreakHitResult _array_element_2))))
        (CallFunction|ApplyDamage (Ability|GetAbilitySystemComponent (.HitActor (Collision|BreakHitResult _array_element_2))))))))

(fn ConstructionScript
  (|CallParentFunction))

(fn GetNoneTargetSpawnLocation
  (bind _caller (Variables|Default|GetCaller))
  (bind _returnvalue (Transformation|GetActorForwardVector _caller))
  (bind _returnvalue_2 (Transformation|GetActorLocation _caller))
  (bind _returnvalue_3 (* _returnvalue 1e+03))
  (bind _returnvalue_4 (+ _returnvalue_2 _returnvalue_3))
  (bind (_outhit _returnvalue_5) (Collision|LineTraceByChannel _returnvalue_2 _returnvalue_4 "TraceTypeQuery1" false (Utilities|Array|MakeArray _caller) "None"))
  (if _returnvalue_5
    (return (.Location (Collision|BreakHitResult _outhit)))
    (else
      (return _returnvalue_4))))