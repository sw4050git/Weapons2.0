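; BP_MagicActor_Fireball is a short-lived magic actor that launches a fireball on behalf of its Caller.
; On BeginPlay, if the Caller is valid, it gets the hand location and target actor through messages to the Caller.
; It spawns BP_FIreBall at the hand, aimed at the target or using its own rotation when there is none.
; It passes the Caller to the fireball, then destroys itself.
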(event EventBeginPlay
  (|CallParentFunction)
  (Utilities|IsValid (Variables|Default|GetCaller)
    (:Is%20Valid
      (bind _handlocation (Class|BPIFCharacterBase|GetHandLocation(Message) (Variables|Default|GetCaller)))
      (Variables|Default|SetHand%20Location _handlocation)
      (bind _targetactor (Class|BPIFPlayer|GetTargetActor(Message) (Variables|Default|GetCaller)))
      (Utilities|IsValid _targetactor
        (:Is%20Valid
          (Game|SpawnActorfromClass "/Game/Game/Blueprints/Stuff/Item/Magic/BP_FIreBall.BP_FIreBall_C" (Math|Transform|MakeTransform (Variables|Default|GetHand%20Location) (Math|Rotator|FindLookatRotation (Variables|Default|GetHand%20Location) (Transformation|GetActorLocation _targetactor)) "1.000000,1.000000,1.000000") "Undefined" "MultiplyWithRoot" 0 (Variables|Default|GetCaller) 0))
        (:Is%20Not%20Valid
          (Game|SpawnActorfromClass "/Game/Game/Blueprints/Stuff/Item/Magic/BP_FIreBall.BP_FIreBall_C" (Math|Transform|MakeTransform (Variables|Default|GetHand%20Location) (Transformation|GetActorRotation) "1.000000,1.000000,1.000000") "Undefined" "MultiplyWithRoot" 0 (Variables|Default|GetCaller) 0)))
      (Actor|DestroyActor))))

(fn ConstructionScript
  (|CallParentFunction))