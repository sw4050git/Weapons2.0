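; BP_FIreBall is a magic fireball actor that damages Attackable actors on sphere overlap, ignoring its Caller.
; Damage reuses the GAS health recovery effect with a negative SetByCaller magnitude, created and applied through the victim's own ability system component.
; Any non-Caller overlap spawns a fire impact effect, disables collision and stops Niagara spawning, then destroys the actor after a delay so particles can fade.
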(event OnComponentBeginOverlap(Sphere)
  (params (OverlappedComponent :type Primitive%20Component%20Object%20Reference) (OtherActor :type Actor%20Object%20Reference) (OtherComp :type Primitive%20Component%20Object%20Reference) (OtherBodyIndex :type Integer) (bFromSweep :type Boolean) (SweepResult :type Hit%20Result%20Structure%20%28by%20ref%29))
  (bind _returnvalue (Ability|GetAbilitySystemComponent OtherActor))
  (if (!= OtherActor (Variables|Default|GetCaller))
    (if (Actor|ActorHasTag OtherActor "Attackable")
      (bind _returnvalue_2 (Ability|GameplayEffect|AssignTagSetbyCallerMagnitude (GameplayEffects|MakeOutgoingSpec :self _returnvalue :GameplayEffectClass "/Game/Game/Blueprints/GameplayEffect/Health/GPE_Health_Recover.GPE_Health_Recover_C") "(TagName=\"Effect.Recover.Health\")" -2e+01))
      (GameplayEffects|ApplyGameplayEffectSpecToTarget _returnvalue _returnvalue_2 _returnvalue))
    (Niagara|SpawnSystematLocation "/Game/Assets/K3/VFX/VFX_Fireball/NS_Fire_Damage.NS_Fire_Damage" (Transformation|GetActorLocation) (Transformation|GetActorRotation))
    (Collision|SetCollisionEnabled (Variables|Default|GetSphere) "NoCollision")
    (Niagara|SetNiagaraVariable(Float) (Variables|Default|GetNiagara) "SpawnRate" 0.0)
    (Utilities|FlowControl|Delay 4.0)
    (Actor|DestroyActor)))

(fn ConstructionScript)